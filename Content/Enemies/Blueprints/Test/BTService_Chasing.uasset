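; Behavior tree service that picks the enemy's ChaseTarget on the blackboard each tick.
; When hasSeenPlayer is set and the BP_EnemyBase_Test pawn is not attacking, the target is the player character.
; Otherwise, if the player is unseen or the enemy is attacking, the target is the pawn itself so it stays put.
; Debug prints report "chase" or "stay".
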(event EventReceiveTickAI
  (params (OwnerController :type AI%20Controller%20Object%20Reference) (ControlledPawn :type Pawn%20Object%20Reference) (DeltaSeconds :type Float%20%28single-precision%29))
  (bind _returnvalue (Utilities|Name|MakeLiteralName "ChaseTarget"))
  (bind _returnvalue_2 (AI|GetBlackboard OwnerController))
  (if (ScalableFloat|GetValueasBool (AI|GetBlackboard OwnerController) (Utilities|Name|MakeLiteralName "hasSeenPlayer"))
    (bind _asbp_enemy_base_test (Utilities|Casting|CastToBP_EnemyBase_Test ControlledPawn))
    (if (Variables|/Game/Enemies/Blueprints/Test/BP_EnemyBase_Test.BP_EnemyBase_Test_C|GetIs%20Attacking _asbp_enemy_base_test)
      ;[1 1 1] not chase
      (AI|Components|Blackboard|SetValueasObject _returnvalue_2 _returnvalue ControlledPawn :!label _label)
      (Development|PrintString "stay")
      (else
        ;[1 1 1] Chase Player
        (AI|Components|Blackboard|SetValueasObject _returnvalue_2 _returnvalue (Game|GetPlayerCharacter 0))
        (Development|PrintString "chase")))
    (else
      (goto _label))))