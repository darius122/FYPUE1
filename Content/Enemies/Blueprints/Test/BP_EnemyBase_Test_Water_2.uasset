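; BP_EnemyBase_Test_Water_2 is a test water enemy Blueprint that adds a head actor and scales its health on BeginPlay.
; After running the parent logic, it spawns a BP_EnemyHeadWater and snaps it to the mesh's head socket.
; It then raises max health by a fixed bonus per HeadCount and sets current health to that new maximum.
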(event EventBeginPlay
  (|CallParentFunction)
  (bind _returnvalue (Game|SpawnActorfromClass "/Game/Enemies/Blueprints/BP_EnemyHeadWater.BP_EnemyHeadWater_C" (Transformation|GetSocketTransform (Variables|Character|GetMesh) "Head_jntSocket" "RTS_World") "AlwaysSpawn" 0 0))
  (Transformation|AttachComponentToComponent _returnvalue (Variables|Character|GetMesh) "Head_jntSocket" "SnapToTarget" "SnapToTarget" "SnapToTarget" true)
  (bind _output_get (Variables|Default|SetEnemyMaxHealth (+ (Variables|Default|GetEnemyMaxHealth) (* 10 (Variables|Default|GetHeadCount)))))
  (Variables|Default|SetEnemyHealth _output_get))

(fn ConstructionScript
  (|CallParentFunction))