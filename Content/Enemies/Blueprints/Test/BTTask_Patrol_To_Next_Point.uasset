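; Behavior tree task that sends a BP_EnemyBase_Test enemy to the next point in its assigned patrol area.
; On successful arrival it updates the enemy's last passed point number and finishes successfully; a failed move never finishes the task.
; Without a valid area or points, it starts a move to a random nearby reachable location, then finishes as failed after a short delay without waiting for arrival.
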(event EventReceiveExecuteAI
  (params (OwnerController :type AI%20Controller%20Object%20Reference) (ControlledPawn :type Pawn%20Object%20Reference))
  (bind _asbp_enemy_base_test (Utilities|Casting|CastToBP_EnemyBase_Test ControlledPawn))
  ;[1 1 1] Is Area there?
  (if (Utilities|IsValid (Variables|/Game/Enemies/Blueprints/Test/BP_EnemyBase_Test.BP_EnemyBase_Test_C|GetMy%20Patrol%20Area _asbp_enemy_base_test))
    ;[1 1 1] Are Points there?
    (if (> (Variables|/Game/Enemies/Blueprints/Test/BP_Patrol_Area.BP_Patrol_Area_C|GetAll%20Points%20Number (Variables|/Game/Enemies/Blueprints/Test/BP_EnemyBase_Test.BP_EnemyBase_Test_C|GetMy%20Patrol%20Area _asbp_enemy_base_test)) 0)
      (AI|AIMoveTo _asbp_enemy_base_test (Transformation|GetActorLocation (Default|GetNextPoint (Variables|/Game/Enemies/Blueprints/Test/BP_EnemyBase_Test.BP_EnemyBase_Test_C|GetMy%20Patrol%20Area _asbp_enemy_base_test) (Variables|/Game/Enemies/Blueprints/Test/BP_EnemyBase_Test.BP_EnemyBase_Test_C|GetLast%20Passed%20Point%20Number _asbp_enemy_base_test))) 0 1.2e+02 false
        (:OnSuccess
          (Variables|/Game/Enemies/Blueprints/Test/BP_EnemyBase_Test.BP_EnemyBase_Test_C|SetLast%20Passed%20Point%20Number _asbp_enemy_base_test (Default|GetNextPointNumber (Variables|/Game/Enemies/Blueprints/Test/BP_EnemyBase_Test.BP_EnemyBase_Test_C|GetMy%20Patrol%20Area _asbp_enemy_base_test) (Variables|/Game/Enemies/Blueprints/Test/BP_EnemyBase_Test.BP_EnemyBase_Test_C|GetLast%20Passed%20Point%20Number _asbp_enemy_base_test)))
          (AI|BehaviorTree|FinishExecute true)))
      (else
        ;[1 1 1] Random Move
        (AI|AIMoveTo _asbp_enemy_base_test (.RandomLocation (AI|Navigation|GetRandomReachablePointinRadius (Transformation|GetActorLocation _asbp_enemy_base_test) 1e+03 0 0)) 0 1.2e+02 false :!label _label
          (:then
            (Utilities|FlowControl|Delay 2.0)
            (AI|BehaviorTree|FinishExecute false)))))
    (else
      (goto _label))))