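; Test enemy variant that gives the base enemy an electric head.
; On BeginPlay it runs the parent logic, spawns a scaled BP_EnemyHeadElectric actor and attaches it to the mesh's neck socket, keeping its world rotation.
; It then raises max health by a bonus per HeadCount and sets current health to that maximum.
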(event EventBeginPlay
  (|CallParentFunction)
  (bind _returnvalue (Game|SpawnActorfromClass "/Game/Enemies/Blueprints/BP_EnemyHeadElectric.BP_EnemyHeadElectric_C" (Math|Transform|MakeTransform (Transformation|GetSocketLocation (Variables|Character|GetMesh) "Neck_jntSocket") "0.000000,-90.000000,0.000000" "1.500000,1.500000,1.500000") "Undefined" 0 0))
  (Transformation|AttachComponentToComponent _returnvalue (Variables|Character|GetMesh) "Neck_jntSocket" "SnapToTarget" "KeepWorld" "KeepRelative" true)
  (bind _output_get (Variables|Default|SetEnemyMaxHealth (+ (Variables|Default|GetEnemyMaxHealth) (* 10 (Variables|Default|GetHeadCount)))))
  (Variables|Default|SetEnemyHealth _output_get))

(event Collision|EventActorBeginOverlap
  (params (OtherActor :type Actor%20Object%20Reference)))

(event EventTick
  (params (DeltaSeconds :type Float%20%28single-precision%29))
  (|CallParentFunction DeltaSeconds) ; This node is disabled and will not be called.\nDrag off pins to build functionality.
)

(fn ConstructionScript
  (|CallParentFunction))