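; Test enemy spawner that spawns an AI enemy about once per second while fewer than 50 enemies exist.
; Tick counts time, then picks a random spawn point actor and offsets the location in X and Y within its radius, giving a square area.
; Each spawned test enemy runs a behavior tree and gets one of three random elements, copied to its head, which then changes colour to match.
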(event Custom|Spawn
  (params (Location :type Vector))
  (bind _returnvalue (AI|SpawnAIFromClass "/Game/Enemies/Blueprints/Test/BP_EnemyBase_Test.BP_EnemyBase_Test_C" "/Game/Enemies/Blueprints/Test/BT_AI1.BT_AI1" Location "0, 0, 0" false 0))
  ;[1 1 1] Change element and color
  (bind _asbp_enemy_base (Utilities|Casting|CastToBP_EnemyBase _returnvalue))
  (Utilities|FlowControl|Sequence
    (:then_0
      (switch int (Math|Random|RandomIntegerinRange 0 2)
        (:0
          (bind _output_get (Variables|/Game/Enemies/Blueprints/BP_EnemyBase.BP_EnemyBase_C|SetElement _asbp_enemy_base "NewEnumerator0"))
          (Variables|/Game/Enemies/Blueprints/BP_EnemyHeadBase.BP_EnemyHeadBase_C|SetElement (Variables|/Game/Enemies/Blueprints/BP_EnemyBase.BP_EnemyBase_C|GetEnemy%20Head%20REF _asbp_enemy_base) _output_get))
        (:1
          (bind _output_get_2 (Variables|/Game/Enemies/Blueprints/BP_EnemyBase.BP_EnemyBase_C|SetElement _asbp_enemy_base "NewEnumerator1"))
          (Variables|/Game/Enemies/Blueprints/BP_EnemyHeadBase.BP_EnemyHeadBase_C|SetElement (Variables|/Game/Enemies/Blueprints/BP_EnemyBase.BP_EnemyBase_C|GetEnemy%20Head%20REF _asbp_enemy_base) _output_get_2))
        (:2
          (bind _output_get_3 (Variables|/Game/Enemies/Blueprints/BP_EnemyBase.BP_EnemyBase_C|SetElement _asbp_enemy_base "NewEnumerator2"))
          (Variables|/Game/Enemies/Blueprints/BP_EnemyHeadBase.BP_EnemyHeadBase_C|SetElement (Variables|/Game/Enemies/Blueprints/BP_EnemyBase.BP_EnemyBase_C|GetEnemy%20Head%20REF _asbp_enemy_base) _output_get_3))))
    (:then_1
      (Default|ChangeColour (Variables|/Game/Enemies/Blueprints/BP_EnemyBase.BP_EnemyBase_C|GetEnemy%20Head%20REF _asbp_enemy_base)))))

(event Custom|Select%20Spawn%20Prace
  ;[1 1 1] Randomly select from SpawnPoints
  (bind _outactors (Actor|GetAllActorsOfClass "/Game/Enemies/Blueprints/Test/BP_EnemySpawn_Point.BP_EnemySpawn_Point_C"))
  (if (> (Utilities|Array|Length _outactors) 0)
    (CallFunction|Spawn (+ (Transformation|GetActorLocation (Utilities|Array|Get(acopy) _outactors (Math|Random|RandomIntegerinRange 0 (- (Utilities|Array|Length _outactors) 1)))) (Math|Vector|MakeVector (Math|Random|RandomFloatinRange (* (Variables|/Game/Enemies/Blueprints/Test/BP_EnemySpawn_Point.BP_EnemySpawn_Point_C|GetRadius (Utilities|Array|Get(acopy) _outactors (Math|Random|RandomIntegerinRange 0 (- (Utilities|Array|Length _outactors) 1)))) -1e+02) (* (Variables|/Game/Enemies/Blueprints/Test/BP_EnemySpawn_Point.BP_EnemySpawn_Point_C|GetRadius (Utilities|Array|Get(acopy) _outactors (Math|Random|RandomIntegerinRange 0 (- (Utilities|Array|Length _outactors) 1)))) 1e+02)) (Math|Random|RandomFloatinRange (* (Variables|/Game/Enemies/Blueprints/Test/BP_EnemySpawn_Point.BP_EnemySpawn_Point_C|GetRadius (Utilities|Array|Get(acopy) _outactors (Math|Random|RandomIntegerinRange 0 (- (Utilities|Array|Length _outactors) 1)))) -1e+02) (* (Variables|/Game/Enemies/Blueprints/Test/BP_EnemySpawn_Point.BP_EnemySpawn_Point_C|GetRadius (Utilities|Array|Get(acopy) _outactors (Math|Random|RandomIntegerinRange 0 (- (Utilities|Array|Length _outactors) 1)))) 1e+02)) 0.0)))))

(event EventBeginPlay)

(event EventTick
  (params (DeltaSeconds :type Float%20%28single-precision%29))
  ;[1 1 1] Less than limit
  (bind _outactors (Actor|GetAllActorsOfClass "/Game/Enemies/Blueprints/BP_EnemyBase.BP_EnemyBase_C"))
  (if (< (Utilities|Array|Length _outactors) 50)
    ;[1 1 1] Count Spawn Time
    (bind _output_get (Variables|Default|SetSpawn%20Time (+ (stale _output_get) DeltaSeconds)))
    (if (>= _output_get 1.0)
      (Variables|Default|SetSpawn%20Time 0.0)
      (CallFunction|SelectSpawnPrace))))

(fn ConstructionScript)