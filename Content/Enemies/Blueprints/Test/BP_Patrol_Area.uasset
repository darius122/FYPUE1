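; Patrol area actor that manages a looping sequence of BP_Patrol_Point actors, in an enemy test folder.
; On BeginPlay it gathers every patrol point in the level, rather than only its own, and numbers each by array index.
; Lookup functions return the next point or number, wrapping to the first after the last.
; Construction-script logic for spawning numbered, parented child points is disconnected and never runs.
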(event EventBeginPlay
  ;[1 1 1] All Points
  (bind _outactors (Actor|GetAllActorsOfClass "/Game/Enemies/Blueprints/Test/BP_Patrol_Point.BP_Patrol_Point_C"))
  (bind _output_get (Variables|Default|SetChaileren%20of%20Point _outactors))
  (for (_array_element _array_index) _output_get
    (Variables|/Game/Enemies/Blueprints/Test/BP_Patrol_Point.BP_Patrol_Point_C|SetNumber _array_element _array_index))
  (Variables|Default|SetAll%20Points%20Number (Utilities|Array|Length (Variables|Default|GetChaileren%20of%20Point))))

(fn ConstructionScript)

(fn GetNextPointNumber
  (params (Now%20Point :type Integer))
  (if (>= Now%20Point (- (Variables|Default|GetAll%20Points%20Number) 1))
    (return 0)
    (else
      (return (+ Now%20Point 1)))))

(fn GetNextPoint
  (params (Now%20Point :type Integer))
  (return (Utilities|Array|Get(acopy) (Variables|Default|GetChaileren%20of%20Point) (CallFunction|GetNextPointNumber Now%20Point))))