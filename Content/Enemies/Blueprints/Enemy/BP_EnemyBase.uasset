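; Base enemy with an element and a stack of elemental heads that serve as extra health.
; AddEnemyHead attaches and offsets Fire, Water or Electricity heads, then SetHealth recalculates health from HeadCount.
; Damage detaches heads as physics objects; death drops the rest, enables mesh physics, may drop a battery and poofs.
; CheckReaction turns mixed elements into an explosion, air current or puddle scaled by HeadCount, destroying enemy and heads.
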(event Custom|ShowHitEffect
  (params (Location :type Vector))
  (bind _returnvalue (AddComponent|AddWidgetComponent true (Math|Transform|MakeTransform Location "0, 0, 0" "1.000000,1.000000,1.000000")))
  (Utilities|FlowControl|Delay 0.2)
  (Components|DestroyComponent _returnvalue))

(event Custom|ShowHeadPopOffEffect
  (params (Location :type Vector))
  (bind _returnvalue (AddComponent|AddWidgetComponent true (Math|Transform|MakeTransform Location "0, 0, 0" "1.000000,1.000000,1.000000")))
  (Utilities|FlowControl|Delay 0.5)
  (Components|DestroyComponent _returnvalue))

(event Collision|EventHit
  (params (MyComp :type Primitive%20Component%20Object%20Reference) (Other :type Actor%20Object%20Reference) (OtherComp :type Primitive%20Component%20Object%20Reference) (bSelfMoved :type Boolean) (HitLocation :type Vector :default "0, 0, 0") (HitNormal :type Vector :default "0, 0, 0") (NormalImpulse :type Vector :default "0, 0, 0") (Hit :type Hit%20Result%20Structure%20%28by%20ref%29)))

(event Game|Damage|EventAnyDamage
  (params (Damage :type Float%20%28single-precision%29) (DamageType :type Damage%20Type%20Object%20Reference) (InstigatedBy :type Controller%20Object%20Reference) (DamageCauser :type Actor%20Object%20Reference))
  (bind _mesh (Variables|Character|GetMesh))
  (bind _children (Components|GetChildrenComponents _mesh false))
  (if (> (- (Variables|Default|GetEnemyHealth) Damage) 0.0)
    (Variables|Default|SetEnemyHealth (Math|Float|Clamp(Float) (- (Variables|Default|GetEnemyHealth) Damage) 0.0 (Variables|Default|GetEnemyMaxHealth)))
    (if (> (Variables|Default|GetHeadCount) 0)
      (CallFunction|DropHead (Math|Float|Truncate Damage)))
    (elif (> (Utilities|Array|Length _children) 0)
      (bind _arrayelement (Utilities|Array|ReverseforEachLoop _children)
        (:LoopBody
          (bind _asbp_enemy_head_base (Utilities|Casting|CastToBP_EnemyHeadBase (Components|GetOwner _arrayelement)))
          (Transformation|DetachFromComponent (Variables|/Script/Engine.Actor|GetRootComponent _asbp_enemy_head_base) "KeepRelative" "KeepRelative" "KeepRelative" true)
          (Physics|SetSimulatePhysics (Variables|/Game/Enemies/Blueprints/EnemyHead/BP_EnemyHeadBase.BP_EnemyHeadBase_C|GetHead _asbp_enemy_head_base) true))
        (:Completed
          (Utilities|FlowControl|DoOnce false :!label _label
            (:Completed
              (Physics|SetSimulatePhysics (Variables|Character|GetMesh) true)
              (CallFunction|DropLoot)
              (Utilities|FlowControl|Delay 2.0)
              (bind _returnvalue (Niagara|SpawnSystematLocation "/Game/Effects/NE_Poof.NE_Poof" (Transformation|GetActorLocation)))
              (Effects|Components|ParticleSystem|SetColorParameter _returnvalue "Color_01" (Variables|Default|GetColor1))
              (Effects|Components|ParticleSystem|SetColorParameter _returnvalue "Color_02" (Variables|Default|GetColor2))
              (Actor|DestroyActor)))))
      (else
        (goto _label)))))

(event EventBeginPlay)

(fn ConstructionScript)

(fn AddEnemyHead
  (params (HeadElement :type Element%20Enum :default "NewEnumerator0"))
  (bind _mesh (Variables|Character|GetMesh))
  (bind _mesh_2 (Variables|Character|GetMesh))
  (bind _mesh_3 (Variables|Character|GetMesh))
  (bind _mesh_4 (Variables|Character|GetMesh))
  (bind _children (Components|GetChildrenComponents _mesh_2 false))
  (bind _children_2 (Components|GetChildrenComponents _mesh_4 false))
  (bind _children_3 (Components|GetChildrenComponents _mesh_3 false))
  (bind _returnvalue (Transformation|GetSocketTransform _mesh "Head_jntSocket" "RTS_World"))
  (switch Utilities|FlowControl|Switch|SwitchonElement HeadElement
    (:NewEnumerator0
      (bind _returnvalue_2 (Game|SpawnActorfromClass "/Game/Enemies/Blueprints/EnemyHead/BP_EnemyHeadFire.BP_EnemyHeadFire_C" _returnvalue "AlwaysSpawn" 0 0))
      (Utilities|IsValid _returnvalue_2
        (:Is%20Valid
          (if (> (Variables|Default|GetHeadCount) 0)
            (Transformation|AttachComponentToComponent _returnvalue_2 (Variables|Character|GetMesh) "Head_jntSocket" "SnapToTarget" "SnapToTarget" "SnapToTarget" true)
            (Transformation|SetActorLocation _returnvalue_2 (+ (Transformation|GetWorldLocation (Utilities|Array|Get(acopy) _children (Utilities|Array|LastIndex _children))) (Math|Vector|MakeVector 0.0 0.0 (* (Variables|Default|GetHeadCount) (LocalVariables|GetHead%20Offset)))) false false)
            (else
              (Transformation|AttachComponentToComponent _returnvalue_2 (Variables|Character|GetMesh) "Head_jntSocket" "SnapToTarget" "SnapToTarget" "SnapToTarget" true))))))
    (:NewEnumerator1
      (bind _returnvalue_3 (Game|SpawnActorfromClass "/Game/Enemies/Blueprints/EnemyHead/BP_EnemyHeadWater.BP_EnemyHeadWater_C" _returnvalue "AlwaysSpawn" 0 0))
      (Utilities|IsValid _returnvalue_3
        (:Is%20Valid
          (if (> (Variables|Default|GetHeadCount) 0)
            (Transformation|AttachComponentToComponent _returnvalue_3 (Variables|Character|GetMesh) "Head_jntSocket" "SnapToTarget" "SnapToTarget" "SnapToTarget" true)
            (Transformation|SetActorLocation _returnvalue_3 (+ (Transformation|GetWorldLocation (Utilities|Array|Get(acopy) _children_2 (Utilities|Array|LastIndex _children_2))) (Math|Vector|MakeVector 0.0 0.0 (* (Variables|Default|GetHeadCount) (LocalVariables|GetHead%20Offset)))) false false)
            (else
              (Transformation|AttachComponentToComponent _returnvalue_3 (Variables|Character|GetMesh) "Head_jntSocket" "SnapToTarget" "SnapToTarget" "SnapToTarget" true))))))
    (:NewEnumerator2
      (bind _returnvalue_4 (Game|SpawnActorfromClass "/Game/Enemies/Blueprints/EnemyHead/BP_EnemyHeadElectric.BP_EnemyHeadElectric_C" _returnvalue "AlwaysSpawn" 0 0))
      (Utilities|IsValid _returnvalue_4
        (:Is%20Valid
          (if (> (Variables|Default|GetHeadCount) 0)
            (Transformation|AttachComponentToComponent _returnvalue_4 (Variables|Character|GetMesh) "Head_jntSocket" "SnapToTarget" "SnapToTarget" "SnapToTarget" true)
            (Transformation|SetActorLocation _returnvalue_4 (+ (Transformation|GetWorldLocation (Utilities|Array|Get(acopy) _children_3 (Utilities|Array|LastIndex _children_3))) (Math|Vector|MakeVector 0.0 0.0 (* (Variables|Default|GetHeadCount) (LocalVariables|GetHead%20Offset)))) false false)
            (else
              (Transformation|AttachComponentToComponent _returnvalue_4 (Variables|Character|GetMesh) "Head_jntSocket" "SnapToTarget" "SnapToTarget" "SnapToTarget" true)))))))
  (Utilities|SetHealth))

(fn CheckReaction
  (params (HeadElement :type Element%20Enum :default "NewEnumerator0"))
  (bind _returnvalue (Transformation|GetActorLocation))
  (bind _returnvalue_2 (Transformation|GetActorLocation))
  (bind _returnvalue_3 (Transformation|GetActorLocation))
  (bind _returnvalue_4 (+ _returnvalue_2 "0.000000,0.000000,150.000000"))
  (bind _returnvalue_5 (+ _returnvalue_3 "0.000000,0.000000,-50.000000"))
  (bind _output_get (Variables|Default|SetHead%20Element HeadElement))
  (if (== (Math|Conversions|ToInteger(Byte) _output_get) (Math|Conversions|ToInteger(Byte) (Variables|Default|GetElement)))
    (Development|PrintString "same element")
    (elif (or (and (== (Math|Conversions|ToInteger(Byte) (Variables|Default|GetElement)) (Math|Conversions|ToInteger(Byte) (Utilities|Enum|LiteralenumElement "NewEnumerator0"))) (== (Math|Conversions|ToInteger(Byte) (Variables|Default|GetHead%20Element)) (Math|Conversions|ToInteger(Byte) (Utilities|Enum|LiteralenumElement "NewEnumerator2")))) (and (== (Math|Conversions|ToInteger(Byte) (Variables|Default|GetHead%20Element)) (Math|Conversions|ToInteger(Byte) (Utilities|Enum|LiteralenumElement "NewEnumerator0"))) (== (Math|Conversions|ToInteger(Byte) (Variables|Default|GetElement)) (Math|Conversions|ToInteger(Byte) (Utilities|Enum|LiteralenumElement "NewEnumerator2")))))
      ;[1 1 1] Fire + Electricity = Explosion
      (Rendering|Debug|DrawDebugSphere _returnvalue (Math|Conversions|ToFloat(Integer) (* 150 (Variables|Default|GetHeadCount))) 12 "(R=0.100625,G=0.000000,B=1.000000,A=1.000000)" 5.0)
      (bind _outactors (Collision|SphereOverlapActors _returnvalue (Math|Conversions|ToFloat(Integer) (* 150 (Variables|Default|GetHeadCount))) (Utilities|Array|MakeArray "ObjectTypeQuery3") 0))
      (Effects|SpawnEmitteratLocation "/Game/StarterContent/Particles/P_Explosion.P_Explosion" _returnvalue "0, 0, 0" "3.000000,3.000000,3.000000")
      (Variables|Default|SetHeadCount 0)
      (for _array_element _outactors
        (bind _asbp_box (Utilities|Casting|CastToBP_Box _array_element)
          (:then
            (bind _box_geo (Default|DestroyBox _asbp_box))
            (Default|Explode _box_geo)
            ;[1 1 1] destroy all heads that are reacted with
            (bind _arrayelement (Utilities|Array|ReverseforEachLoop (Components|GetChildrenComponents (Variables|Character|GetMesh) false))
              (:LoopBody
                (bind _asbp_enemy_head_base (Utilities|Casting|CastToBP_EnemyHeadBase (Components|GetOwner _arrayelement)))
                (Actor|DestroyActor _asbp_enemy_head_base))
              (:Completed
                (Actor|DestroyActor))))
          (:CastFailed
            (Game|Damage|ApplyDamage _array_element 3e+01 0 self))))
      (bind _arrayelement_2 (Utilities|Array|ReverseforEachLoop (Components|GetChildrenComponents (Variables|Character|GetMesh) false))
        (:LoopBody
          (bind _asbp_enemy_head_base_2 (Utilities|Casting|CastToBP_EnemyHeadBase (Components|GetOwner _arrayelement_2)))
          (Actor|DestroyActor _asbp_enemy_head_base_2))
        (:Completed
          (Actor|DestroyActor)))
      (elif (or (and (== (Math|Conversions|ToInteger(Byte) (Variables|Default|GetElement)) (Math|Conversions|ToInteger(Byte) (Utilities|Enum|LiteralenumElement "NewEnumerator0"))) (== (Math|Conversions|ToInteger(Byte) (Variables|Default|GetHead%20Element)) (Math|Conversions|ToInteger(Byte) (Utilities|Enum|LiteralenumElement "NewEnumerator1")))) (and (== (Math|Conversions|ToInteger(Byte) (Variables|Default|GetHead%20Element)) (Math|Conversions|ToInteger(Byte) (Utilities|Enum|LiteralenumElement "NewEnumerator0"))) (== (Math|Conversions|ToInteger(Byte) (Variables|Default|GetElement)) (Math|Conversions|ToInteger(Byte) (Utilities|Enum|LiteralenumElement "NewEnumerator1")))))
        ;[1 1 1] Fire + Water = Air Current
        (bind _returnvalue_6 (Game|SpawnActorfromClass "/Game/FirstPerson/Blueprints/Reactions/BP_AirCurrent.BP_AirCurrent_C" (Transformation|GetActorTransform) "Undefined" 0 0))
        (Transformation|SetActorLocation _returnvalue_6 _returnvalue_4 false false)
        ;[1 1 1] destroy all heads that are reacted with
        (Transformation|SetActorScale3D _returnvalue_6 (Math|Vector|MakeVector (+ (* (Math|Float|MakeLiteralFloat 0.75) (Variables|Default|GetHeadCount)) (.x (Transformation|GetActorScale3D _returnvalue_6))) (+ (* (Math|Float|MakeLiteralFloat 0.75) (Variables|Default|GetHeadCount)) (.x (Transformation|GetActorScale3D _returnvalue_6))) (+ (* (Math|Float|MakeLiteralFloat 1.0) (Variables|Default|GetHeadCount)) (.z (Transformation|GetActorScale3D _returnvalue_6)))))
        (Effects|SpawnEmitteratLocation "/Game/StarterContent/Particles/P_Steam_Lit.P_Steam_Lit" _returnvalue_4 "0, 0, 0" "3.000000,3.000000,5.000000")
        (Variables|Default|SetHeadCount 0)
        (bind _arrayelement_3 (Utilities|Array|ReverseforEachLoop (Components|GetChildrenComponents (Variables|Character|GetMesh) false))
          (:LoopBody
            (bind _asbp_enemy_head_base_3 (Utilities|Casting|CastToBP_EnemyHeadBase (Components|GetOwner _arrayelement_3)))
            (Actor|DestroyActor _asbp_enemy_head_base_3))
          (:Completed
            (Actor|DestroyActor)))
        (else
          ;[1 1 1] Water + Electrivity = Electric puddle
          (if (or (and (== (Math|Conversions|ToInteger(Byte) (Variables|Default|GetElement)) (Math|Conversions|ToInteger(Byte) (Utilities|Enum|LiteralenumElement "NewEnumerator1"))) (== (Math|Conversions|ToInteger(Byte) (Variables|Default|GetHead%20Element)) (Math|Conversions|ToInteger(Byte) (Utilities|Enum|LiteralenumElement "NewEnumerator2")))) (and (== (Math|Conversions|ToInteger(Byte) (Variables|Default|GetHead%20Element)) (Math|Conversions|ToInteger(Byte) (Utilities|Enum|LiteralenumElement "NewEnumerator1"))) (== (Math|Conversions|ToInteger(Byte) (Variables|Default|GetElement)) (Math|Conversions|ToInteger(Byte) (Utilities|Enum|LiteralenumElement "NewEnumerator2")))))
            (bind _returnvalue_7 (Game|SpawnActorfromClass "/Game/FirstPerson/Blueprints/Reactions/BP_Puddle.BP_Puddle_C" (Transformation|GetActorTransform) "Undefined" 0 0))
            (Transformation|SetActorLocation _returnvalue_7 _returnvalue_5 false false)
            (Transformation|SetActorScale3D _returnvalue_7 (Math|Vector|MakeVector (+ (* (Math|Float|MakeLiteralFloat 1.25) (Variables|Default|GetHeadCount)) (.x (Transformation|GetActorScale3D _returnvalue_7))) (+ (* (Math|Float|MakeLiteralFloat 1.25) (Variables|Default|GetHeadCount)) (.x (Transformation|GetActorScale3D _returnvalue_7))) (.z (Transformation|GetActorScale3D _returnvalue_7))))
            (Effects|SpawnEmitteratLocation "/Game/StarterContent/Particles/P_Sparks.P_Sparks" _returnvalue_5 "0, 0, 0" "3.000000,3.000000,3.000000")
            (Variables|Default|SetHeadCount 0)
            ;[1 1 1] destroy all heads that are reacted with
            (bind _arrayelement_4 (Utilities|Array|ReverseforEachLoop (Components|GetChildrenComponents (Variables|Character|GetMesh) false))
              (:LoopBody
                (bind _asbp_enemy_head_base_4 (Utilities|Casting|CastToBP_EnemyHeadBase (Components|GetOwner _arrayelement_4)))
                (Actor|DestroyActor _asbp_enemy_head_base_4))
              (:Completed
                (Actor|DestroyActor)))))))))

(fn DropHead
  (params (Damage%20Taken :type Integer))
  (bind _returnvalue (/ Damage%20Taken 10))
  (bind _mesh (Variables|Character|GetMesh))
  (bind _children (Components|GetChildrenComponents _mesh false))
  (bind _output_get (Variables|Default|SetHeads%20To%20Drop _returnvalue))
  (if (> _output_get 0)
    (bind _arrayelement (Utilities|Array|ReverseforEachLoop _children)
      (:LoopBody
        (if (> (Variables|Default|GetHeads%20To%20Drop) 0)
          (bind _asbp_enemy_head_base (Utilities|Casting|CastToBP_EnemyHeadBase (Components|GetOwner _arrayelement)))
          (Transformation|DetachFromComponent (Variables|/Script/Engine.Actor|GetRootComponent _asbp_enemy_head_base) "KeepRelative" "KeepRelative" "KeepRelative" true)
          (Physics|SetSimulatePhysics (Variables|/Game/Enemies/Blueprints/EnemyHead/BP_EnemyHeadBase.BP_EnemyHeadBase_C|GetHead _asbp_enemy_head_base) true)
          (bind _result (Math|Float|DecrementFloat (Math|Conversions|ToFloat(Integer) (Variables|Default|GetHeads%20To%20Drop)))
            (:%20%20
              (Variables|Default|SetHeads%20To%20Drop (Math|Float|Truncate _result))))))
      (:Completed
        (Variables|Default|SetHeadCount (- (Variables|Default|GetHeadCount) _returnvalue))
        (if (< (Variables|Default|GetHeadCount) 0)
          (Variables|Default|SetHeadCount 0))))
    (elif (<= (Variables|Default|GetEnemyHealth) (+ (* (- (Variables|Default|GetHeadCount) 1) 10) 20))
      (Variables|Default|SetHeads%20To%20Drop 1)
      (bind _arrayelement_2 (Utilities|Array|ReverseforEachLoop _children)
        (:LoopBody
          (if (> (Variables|Default|GetHeads%20To%20Drop) 0)
            (bind _asbp_enemy_head_base_2 (Utilities|Casting|CastToBP_EnemyHeadBase (Components|GetOwner _arrayelement_2)))
            (CallFunction|ShowHeadPopOffEffect (+ (Transformation|GetWorldLocation (Variables|/Game/Enemies/Blueprints/EnemyHead/BP_EnemyHeadBase.BP_EnemyHeadBase_C|GetHead _asbp_enemy_head_base_2)) "20.000000,20.000000,0.000000"))
            (Transformation|DetachFromComponent (Variables|/Script/Engine.Actor|GetRootComponent _asbp_enemy_head_base_2) "KeepRelative" "KeepRelative" "KeepRelative" true)
            (Physics|SetSimulatePhysics (Variables|/Game/Enemies/Blueprints/EnemyHead/BP_EnemyHeadBase.BP_EnemyHeadBase_C|GetHead _asbp_enemy_head_base_2) true)
            (bind _result_2 (Math|Float|DecrementFloat (Math|Conversions|ToFloat(Integer) (Variables|Default|GetHeads%20To%20Drop)))
              (:%20%20
                (Variables|Default|SetHeads%20To%20Drop (Math|Float|Truncate _result_2))
                (bind _result_3 (Math|Integer|DecrementInt (Variables|Default|GetHeadCount))
                  (:%20%20
                    (Variables|Default|SetHeadCount _result_3)))))))))))

(fn DropLoot
  (if (Math|Random|RandomBoolwithWeight 0.2)
    (Game|SpawnActorfromClass "/Game/FirstPerson/Blueprints/Interactable_Items/BP_BatterySmall.BP_BatterySmall_C" (Transformation|GetActorTransform) "Undefined" 0 0)))