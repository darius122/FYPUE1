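; BP_EnemySpawn_Point is an enemy spawn point actor that displays its spawn area as flat cylinders.
; The construction script sizes Cylinder to the diameter of SpawnRadius, converting units by dividing by 100.
; Cylinder1 is a thinner disc sized by SpawnRadius multiplied by EnableSpawnRadius.
; The event graph holds only disabled stub events, so this graph contains no spawning logic.
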(event EventBeginPlay)

(event Collision|EventActorBeginOverlap
  (params (OtherActor :type Actor%20Object%20Reference)))

(event EventTick
  (params (DeltaSeconds :type Float%20%28single-precision%29)))

(fn ConstructionScript
  (bind _spawn_radius (Variables|Default|GetSpawn%20Radius))
  (bind _spawn_radius_2 (Variables|Default|GetSpawn%20Radius))
  (bind _enable_spawn_radius (Variables|Default|GetEnable%20Spawn%20Radius))
  (bind _returnvalue (* _spawn_radius_2 2.0))
  (bind _returnvalue_2 (* _spawn_radius _enable_spawn_radius))
  (bind _returnvalue_3 (* _returnvalue_2 2.0))
  (bind _returnvalue_4 (/ _returnvalue 1e+02))
  (bind _returnvalue_5 (/ _returnvalue_3 1e+02))
  (Transformation|SetWorldScale3D (Variables|Default|GetCylinder) (Math|Vector|MakeVector _returnvalue_4 _returnvalue_4 0.1))
  (Transformation|SetWorldScale3D (Variables|Default|GetCylinder1) (Math|Vector|MakeVector _returnvalue_5 _returnvalue_5 0.05)))