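; Timed enemy spawner that populates BP_EnemySpawn_Point locations with Fire, Water or Electric AI enemies.
; On a looping timer it spawns at points linked to active BP_EnemySpawnerTriggers, and at a random offset around points within range of the player.
; Each spawn randomly uses one of the point's two elements to choose the class, respecting the point's SpawnLimit after pruning invalid entries.
; A weighted random roll sets each enemy's melee attack type.
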(event Custom|CustomEvent
  ;[1 1 1] Count Spawn Time
  ;[1 1 1] when player closed
  (bind _outactors (Actor|GetAllActorsOfClass "/Game/Enemies/Blueprints/Enemy/Spawner/BP_EnemySpawnerTrigger.BP_EnemySpawnerTrigger_C"))
  (for _array_element _outactors
    (if (Variables|/Game/Enemies/Blueprints/Enemy/Spawner/BP_EnemySpawnerTrigger.BP_EnemySpawnerTrigger_C|GetIn%20Area _array_element)
      (for _array_element_2 (Variables|/Game/Enemies/Blueprints/Enemy/Spawner/BP_EnemySpawnerTrigger.BP_EnemySpawnerTrigger_C|GetEnemySpawnPoints _array_element)
        (CallFunction|Spawn (Transformation|GetActorLocation _array_element_2) (Variables|/Game/Enemies/Blueprints/Enemy/Spawner/BP_EnemySpawn_Point.BP_EnemySpawn_Point_C|GetElement%201 _array_element_2) (Variables|/Game/Enemies/Blueprints/Enemy/Spawner/BP_EnemySpawn_Point.BP_EnemySpawn_Point_C|GetElement%202 _array_element_2) _array_element_2))))
  (bind _outactors_2 (Actor|GetAllActorsOfClass "/Game/Enemies/Blueprints/Enemy/Spawner/BP_EnemySpawn_Point.BP_EnemySpawn_Point_C"))
  (for (_array_element_3 _array_index) _outactors_2
    (if (<= (- (Math|Vector|VectorLength (- (Transformation|GetActorLocation _array_element_3) (Transformation|GetActorLocation (Game|GetPlayerCharacter 0)))) (Variables|/Game/Enemies/Blueprints/Enemy/Spawner/BP_EnemySpawn_Point.BP_EnemySpawn_Point_C|GetSpawn%20Radius _array_element_3)) (* (Variables|/Game/Enemies/Blueprints/Enemy/Spawner/BP_EnemySpawn_Point.BP_EnemySpawn_Point_C|GetSpawn%20Radius _array_element_3) (Variables|/Game/Enemies/Blueprints/Enemy/Spawner/BP_EnemySpawn_Point.BP_EnemySpawn_Point_C|GetEnable%20Spawn%20Radius _array_element_3)))
      (CallFunction|SelectSpawnPrace _array_index _array_element_3))))

(event Custom|Spawn
  (params (Location :type Vector) (Element%201 :type Element%20Enum :default "NewEnumerator0") (Element%202 :type Element%20Enum :default "NewEnumerator0") (SpanwPoint :type BP%20Enemy%20Spawn%20Point%20Object%20Reference))
  ;[1 1 1] Spawn Enemies
  (Variables|Default|SetSpanw%20Point SpanwPoint)
  (Variables|Default|SetElement%201 Element%201)
  (Variables|Default|SetElement%202 Element%202)
  (Variables|Default|SetLocation Location)
  (for _array_element (Variables|/Game/Enemies/Blueprints/Enemy/Spawner/BP_EnemySpawn_Point.BP_EnemySpawn_Point_C|GetSpawnedEnemies (Variables|Default|GetSpanw%20Point))
    (Utilities|IsValid _array_element
      (:Is%20Not%20Valid
        (Utilities|Array|RemoveItem (Variables|/Game/Enemies/Blueprints/Enemy/Spawner/BP_EnemySpawn_Point.BP_EnemySpawn_Point_C|GetSpawnedEnemies (Variables|Default|GetSpanw%20Point)) _array_element))))
  (switch int (Math|Random|RandomIntegerinRange 0 1)
    (:0
      (if (CallFunction|CheckElement (Variables|Default|GetElement%201) "NewEnumerator0")
        (if (CallFunction|CheckSpawnLimit (Variables|Default|GetSpanw%20Point))
          (bind _returnvalue (AI|SpawnAIFromClass "/Game/Enemies/Blueprints/Enemy/BP_EnemyBase_Test_Fire.BP_EnemyBase_Test_Fire_C" "/Game/Enemies/AI/BT_AI1.BT_AI1" (Variables|Default|GetLocation) "0, 0, 0" false 0))
          (Utilities|Array|Add (Variables|/Game/Enemies/Blueprints/Enemy/Spawner/BP_EnemySpawn_Point.BP_EnemySpawn_Point_C|GetSpawnedEnemies (Variables|Default|GetSpanw%20Point)) _returnvalue)
          (bind _asbp_enemy_base_test_fire (Utilities|Casting|CastToBP_EnemyBase_Test_Fire _returnvalue))
          (CallFunction|RandomMeleeRange _asbp_enemy_base_test_fire))
        (elif (CallFunction|CheckElement (Variables|Default|GetElement%201) "NewEnumerator1")
          (if (CallFunction|CheckSpawnLimit (Variables|Default|GetSpanw%20Point))
            (bind _returnvalue_2 (AI|SpawnAIFromClass "/Game/Enemies/Blueprints/Enemy/BP_EnemyBase_Test_Water_2.BP_EnemyBase_Test_Water_2_C" "/Game/Enemies/AI/BT_AI1.BT_AI1" (Variables|Default|GetLocation) "0, 0, 0" false 0))
            (Utilities|Array|Add (Variables|/Game/Enemies/Blueprints/Enemy/Spawner/BP_EnemySpawn_Point.BP_EnemySpawn_Point_C|GetSpawnedEnemies (Variables|Default|GetSpanw%20Point)) _returnvalue_2)
            (bind _asbp_enemy_base_test_water_2 (Utilities|Casting|CastToBP_EnemyBase_Test_Water_2 _returnvalue_2))
            (CallFunction|RandomMeleeRange _asbp_enemy_base_test_water_2))
          (elif (CallFunction|CheckElement (Variables|Default|GetElement%201) "NewEnumerator2")
            (if (CallFunction|CheckSpawnLimit (Variables|Default|GetSpanw%20Point))
              (bind _returnvalue_3 (AI|SpawnAIFromClass "/Game/Enemies/Blueprints/Enemy/BP_EnemyBase_Test_Electric.BP_EnemyBase_Test_Electric_C" "/Game/Enemies/AI/BT_AI1.BT_AI1" (Variables|Default|GetLocation) "0, 0, 0" false 0))
              (Utilities|Array|Add (Variables|/Game/Enemies/Blueprints/Enemy/Spawner/BP_EnemySpawn_Point.BP_EnemySpawn_Point_C|GetSpawnedEnemies (Variables|Default|GetSpanw%20Point)) _returnvalue_3)
              (bind _asbp_enemy_base_test_electric (Utilities|Casting|CastToBP_EnemyBase_Test_Electric _returnvalue_3))
              (CallFunction|RandomMeleeRange _asbp_enemy_base_test_electric))))))
    (:1
      (if (CallFunction|CheckElement (Variables|Default|GetElement%202) "NewEnumerator0")
        (if (CallFunction|CheckSpawnLimit (Variables|Default|GetSpanw%20Point))
          (bind _returnvalue_4 (AI|SpawnAIFromClass "/Game/Enemies/Blueprints/Enemy/BP_EnemyBase_Test_Fire.BP_EnemyBase_Test_Fire_C" "/Game/Enemies/AI/BT_AI1.BT_AI1" (Variables|Default|GetLocation) "0, 0, 0" false 0))
          (Utilities|Array|Add (Variables|/Game/Enemies/Blueprints/Enemy/Spawner/BP_EnemySpawn_Point.BP_EnemySpawn_Point_C|GetSpawnedEnemies (Variables|Default|GetSpanw%20Point)) _returnvalue_4)
          (bind _asbp_enemy_base_test_fire_2 (Utilities|Casting|CastToBP_EnemyBase_Test_Fire _returnvalue_4))
          (CallFunction|RandomMeleeRange _asbp_enemy_base_test_fire_2))
        (elif (CallFunction|CheckElement (Variables|Default|GetElement%202) "NewEnumerator1")
          (if (CallFunction|CheckSpawnLimit (Variables|Default|GetSpanw%20Point))
            (bind _returnvalue_5 (AI|SpawnAIFromClass "/Game/Enemies/Blueprints/Enemy/BP_EnemyBase_Test_Water_2.BP_EnemyBase_Test_Water_2_C" "/Game/Enemies/AI/BT_AI1.BT_AI1" (Variables|Default|GetLocation) "0, 0, 0" false 0))
            (Utilities|Array|Add (Variables|/Game/Enemies/Blueprints/Enemy/Spawner/BP_EnemySpawn_Point.BP_EnemySpawn_Point_C|GetSpawnedEnemies (Variables|Default|GetSpanw%20Point)) _returnvalue_5)
            (bind _asbp_enemy_base_test_water_2_2 (Utilities|Casting|CastToBP_EnemyBase_Test_Water_2 _returnvalue_5))
            (CallFunction|RandomMeleeRange _asbp_enemy_base_test_water_2_2))
          (elif (CallFunction|CheckElement (Variables|Default|GetElement%202) "NewEnumerator2")
            (if (CallFunction|CheckSpawnLimit (Variables|Default|GetSpanw%20Point))
              (bind _returnvalue_6 (AI|SpawnAIFromClass "/Game/Enemies/Blueprints/Enemy/BP_EnemyBase_Test_Electric.BP_EnemyBase_Test_Electric_C" "/Game/Enemies/AI/BT_AI1.BT_AI1" (Variables|Default|GetLocation) "0, 0, 0" false 0))
              (Utilities|Array|Add (Variables|/Game/Enemies/Blueprints/Enemy/Spawner/BP_EnemySpawn_Point.BP_EnemySpawn_Point_C|GetSpawnedEnemies (Variables|Default|GetSpanw%20Point)) _returnvalue_6)
              (bind _asbp_enemy_base_test_electric_2 (Utilities|Casting|CastToBP_EnemyBase_Test_Electric _returnvalue_6))
              (CallFunction|RandomMeleeRange _asbp_enemy_base_test_electric_2))))))))

(event Custom|Select%20Spawn%20Prace
  (params (index :type Integer) (SpawnPoint :type BP%20Enemy%20Spawn%20Point%20Object%20Reference))
  ;[1 1 1] Randomly select from SpawnPoints
  (bind _outactors (Actor|GetAllActorsOfClass "/Game/Enemies/Blueprints/Enemy/Spawner/BP_EnemySpawn_Point.BP_EnemySpawn_Point_C"))
  (CallFunction|Spawn (+ (Transformation|GetActorLocation (Utilities|Array|Get(acopy) _outactors index)) (Math|Vector|MakeVector (Math|Random|RandomFloatinRange (* (Variables|/Game/Enemies/Blueprints/Enemy/Spawner/BP_EnemySpawn_Point.BP_EnemySpawn_Point_C|GetSpawn%20Radius (Utilities|Array|Get(acopy) _outactors index)) -1.0) (* (Variables|/Game/Enemies/Blueprints/Enemy/Spawner/BP_EnemySpawn_Point.BP_EnemySpawn_Point_C|GetSpawn%20Radius (Utilities|Array|Get(acopy) _outactors index)) 1.0)) (Math|Random|RandomFloatinRange (* (Variables|/Game/Enemies/Blueprints/Enemy/Spawner/BP_EnemySpawn_Point.BP_EnemySpawn_Point_C|GetSpawn%20Radius (Utilities|Array|Get(acopy) _outactors index)) -1.0) (* (Variables|/Game/Enemies/Blueprints/Enemy/Spawner/BP_EnemySpawn_Point.BP_EnemySpawn_Point_C|GetSpawn%20Radius (Utilities|Array|Get(acopy) _outactors index)) 1.0)) 0.0)) (Variables|/Game/Enemies/Blueprints/Enemy/Spawner/BP_EnemySpawn_Point.BP_EnemySpawn_Point_C|GetElement%201 (Utilities|Array|Get(acopy) _outactors index)) (Variables|/Game/Enemies/Blueprints/Enemy/Spawner/BP_EnemySpawn_Point.BP_EnemySpawn_Point_C|GetElement%202 (Utilities|Array|Get(acopy) _outactors index)) SpawnPoint))

(event EventBeginPlay
  ;[1 1 1] Count Spawn Time
  (Utilities|Time|SetTimerbyEvent (delegate Custom|CustomEvent) (Variables|Default|GetSpawnInterval) true))

(fn ConstructionScript)

(fn CheckElement
  (params (Element :type Element%20Enum :default "NewEnumerator0") (Literal%20enum :type Element%20Enum :default "NewEnumerator0"))
  (return (== (Math|Conversions|ToInteger(Byte) Element) (Math|Conversions|ToInteger(Byte) Literal%20enum))))

(fn CheckSpawnLimit
  (params (SpawnPoint :type BP%20Enemy%20Spawn%20Point%20Object%20Reference))
  (return (< (Utilities|Array|Length (Variables|/Game/Enemies/Blueprints/Enemy/Spawner/BP_EnemySpawn_Point.BP_EnemySpawn_Point_C|GetSpawnedEnemies SpawnPoint)) (Variables|/Game/Enemies/Blueprints/Enemy/Spawner/BP_EnemySpawn_Point.BP_EnemySpawn_Point_C|GetSpawn%20Limit SpawnPoint))))

(fn RandomMeleeRange
  (params (Return%20Value :type BP%20Enemy%20Base%20Test%20Object%20Reference))
  (Variables|/Game/Enemies/Blueprints/Enemy/BP_EnemyBase_Test.BP_EnemyBase_Test_C|SetAttack%20Type%20Melee Return%20Value (Math|Random|RandomBoolwithWeight (Variables|Default|GetSpawnWeight))))