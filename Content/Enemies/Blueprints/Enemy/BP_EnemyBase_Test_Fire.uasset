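; Test fire variant of an enemy, assembled from attachments on its skeletal mesh when play begins.
; BeginPlay runs the parent logic, then spawns a BP_EnemyHeadFire actor and snaps it to the head socket.
; It raises max health in proportion to HeadCount and sets current health to that maximum.
; A crossbrace component is also snapped to a right middle-finger socket, and the construction script only calls the parent.
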(event EventBeginPlay
  (|CallParentFunction)
  (Utilities|FlowControl|Sequence
    (:then_0
      (bind _returnvalue (Game|SpawnActorfromClass "/Game/Enemies/Blueprints/EnemyHead/BP_EnemyHeadFire.BP_EnemyHeadFire_C" (Transformation|GetSocketTransform (Variables|Character|GetMesh) "Head_jntSocket" "RTS_World") "AlwaysSpawn" 0 0))
      (Transformation|AttachComponentToComponent _returnvalue (Variables|Character|GetMesh) "Head_jntSocket" "SnapToTarget" "SnapToTarget" "SnapToTarget" true)
      (bind _output_get (Variables|Default|SetEnemyMaxHealth (+ (Variables|Default|GetEnemyMaxHealth) (* 10 (Variables|Default|GetHeadCount)))))
      (Variables|Default|SetEnemyHealth _output_get))
    (:then_1
      (Transformation|AttachComponentToComponent (Variables|Default|GetFE_WalkAnim_body_Crossbrace) (Variables|Character|GetMesh) "R_MiddleF_jnt1Socket" "SnapToTarget" "SnapToTarget" "SnapToTarget" true))))

(fn ConstructionScript
  (|CallParentFunction))