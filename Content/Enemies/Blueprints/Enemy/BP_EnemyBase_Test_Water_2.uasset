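; BP_EnemyBase_Test_Water_2 is a water enemy variant that extends its parent's behavior with a head and health setup.
; On BeginPlay, after the parent logic, it spawns a BP_EnemyHeadWater actor and snaps it to the mesh's head socket, keeping world scale.
; It then raises max health in proportion to HeadCount, fills current health to match, and sets two blue color variables.
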(event EventBeginPlay
  (|CallParentFunction)
  (bind _returnvalue (Game|SpawnActorfromClass "/Game/Enemies/Blueprints/EnemyHead/BP_EnemyHeadWater.BP_EnemyHeadWater_C" (Transformation|GetSocketTransform (Variables|Character|GetMesh) "Head_jntSocket" "RTS_World") "AlwaysSpawn" 0 0))
  (Transformation|AttachComponentToComponent _returnvalue (Variables|Character|GetMesh) "Head_jntSocket" "SnapToTarget" "SnapToTarget" "KeepWorld" true)
  (bind _output_get (Variables|Default|SetEnemyMaxHealth (+ (Variables|Default|GetEnemyMaxHealth) (* 10 (Variables|Default|GetHeadCount)))))
  (Variables|Default|SetEnemyHealth _output_get)
  (Variables|Default|SetColor1 "(R=0.000000,G=0.584087,B=1.000000,A=1.000000)")
  (Variables|Default|SetColor2 "(R=0.225118,G=0.450349,B=0.614583,A=1.000000)"))

(fn ConstructionScript
  (|CallParentFunction))