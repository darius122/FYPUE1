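; Boid actor for flocking movement on the XY plane, starting with a random velocity.
; Flock sums weighted alignment, cohesion and separation from sphere-overlap neighbors, plus arrival at world origin, into Acceleration.
; MoveBoid integrates that with a speed clamp, sweeps the actor and rotates its cube.
; Player fleeing, line-trace avoidance and a partial edge clamp are separate functions; nothing here calls them, Flock or MoveBoid.
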(event EventBeginPlay
  (Variables|Default|Setposition (Transformation|GetWorldLocation (Variables|Default|GetCube)))
  (Variables|Default|Setvelocity (Math|Vector|MakeVector (Math|Random|RandomFloatinRange -1e+01 1e+01) (Math|Random|RandomFloatinRange -1e+01 1e+01) 0.0)))

(event Collision|EventActorBeginOverlap
  (params (OtherActor :type Actor%20Object%20Reference)))

(event EventTick
  (params (DeltaSeconds :type Float%20%28single-precision%29)))

(fn ConstructionScript)

(fn MoveBoid
  (bind _output_get (Variables|Default|Setposition (+ (Math|Vector|MakeVector (.x (Variables|Default|Getposition)) (.y (Variables|Default|Getposition)) 0.0) (Math|Vector|MakeVector (.x (Variables|Default|Getvelocity)) (.y (Variables|Default|Getvelocity)) 0.0))))
  (bind _output_get_2 (Variables|Default|Setvelocity (+ (Math|Vector|MakeVector (.x (Variables|Default|Getvelocity)) (.y (Variables|Default|Getvelocity)) 0.0) (Math|Vector|MakeVector (.x (Variables|Default|Getacceleration)) (.y (Variables|Default|Getacceleration)) 0.0))))
  (Variables|Default|Setvelocity (Math|Vector|VectorClampSizeMax _output_get_2 (Variables|Default|GetmaxSpeed)))
  (bind _sweephitresult (Transformation|SetActorLocation _output_get true false))
  (Variables|Default|Setacceleration (* (Variables|Default|Getacceleration) ""))
  (Transformation|SetRelativeRotation (Variables|Default|GetCube) (Math|Rotator|FindLookatRotation (Variables|Default|Getposition) (* (Variables|Default|Getvelocity) 1e+03)) true false))

(fn Align
  (params (Perception%20Radius :type Float%20%28double-precision%29))
  (bind (_outactors _returnvalue) (CallFunction|SphereCast Perception%20Radius))
  (for _array_element _outactors
    (bind _asbp_boid (Utilities|Casting|CastToBP_Boid _array_element))
    (if (and (!= self _array_element) _returnvalue)
      (LocalVariables|Setsteering (+ (Math|Vector|MakeVector (.x (LocalVariables|Getsteering)) (.y (LocalVariables|Getsteering)) 0.0) (Math|Vector|MakeVector (.x (Variables|BP_Boid_C|Getvelocity _asbp_boid)) (.y (Variables|BP_Boid_C|Getvelocity _asbp_boid)) 0.0)))
      (Math|Integer|IncrementInt (LocalVariables|Gettotal))))
  (if (> (LocalVariables|Gettotal) 0)
    (bind _output_get (LocalVariables|Setsteering (/ (LocalVariables|Getsteering) (LocalVariables|Gettotal))))
    (bind _output_get_2 (LocalVariables|Setsteering (- (* (Math|Vector|Normalize _output_get) (Variables|Default|GetmaxSpeed)) (Variables|Default|Getvelocity))))
    (return (Math|Vector|VectorClampSizeMax _output_get_2 (Variables|Default|GetmaxForce)))
    (else
      (return (LocalVariables|Getsteering)))))

(fn Flock
  (params (alignmentMultiplier :type Float%20%28double-precision%29) (cohesionMulitplier :type Float%20%28double-precision%29) (separationMultiplier :type Float%20%28double-precision%29) (alignmentRadius :type Float%20%28double-precision%29) (cohesionRadius :type Float%20%28double-precision%29) (separationRadius :type Float%20%28double-precision%29))
  (LocalVariables|Setalignment (* (CallFunction|Align alignmentRadius) alignmentMultiplier))
  (LocalVariables|Setcohesion (* (CallFunction|Cohesion cohesionRadius) cohesionMulitplier))
  (bind _output_get (LocalVariables|Setseparation (* (CallFunction|Separation separationRadius) separationMultiplier)))
  (bind _output_get_2 (Variables|Default|Setacceleration (+ (Variables|Default|Getacceleration) _output_get)))
  (bind _output_get_3 (Variables|Default|Setacceleration (+ _output_get_2 (LocalVariables|Getalignment))))
  (bind _output_get_4 (Variables|Default|Setacceleration (+ _output_get_3 (LocalVariables|Getcohesion))))
  (Variables|Default|Setacceleration (+ _output_get_4 (* (CallFunction|Arriving) 0.7))))

(fn Edges
  (bind _position (Variables|Default|Getposition))
  (Utilities|FlowControl|Sequence
    (:then_0
      (if (> (.x _position) 4e+03)
        (Class|KismetMathLibrary|VectorSet (Variables|Default|Getposition) 4e+03 (.y _position) (.z _position))))))

(fn Cohesion
  (params (Perception%20Radius :type Float%20%28double-precision%29))
  (bind (_outactors _returnvalue) (CallFunction|SphereCast Perception%20Radius))
  (for _array_element _outactors
    (bind _asbp_boid (Utilities|Casting|CastToBP_Boid _array_element))
    (if (and (!= self _array_element) _returnvalue)
      (LocalVariables|Setsteering (+ (Math|Vector|MakeVector (.x (LocalVariables|Getsteering)) (.y (LocalVariables|Getsteering)) 0.0) (Math|Vector|MakeVector (.x (Variables|BP_Boid_C|Getposition _asbp_boid)) (.y (Variables|BP_Boid_C|Getposition _asbp_boid)) 0.0)))
      (Math|Integer|IncrementInt (LocalVariables|Gettotal))))
  (if (> (LocalVariables|Gettotal) 0)
    (bind _output_get (LocalVariables|Setsteering (/ (LocalVariables|Getsteering) (LocalVariables|Gettotal))))
    (bind _output_get_2 (LocalVariables|Setsteering (- (* (Math|Vector|Normalize _output_get) (Variables|Default|GetmaxSpeed)) (Variables|Default|Getposition))))
    (bind _output_get_3 (LocalVariables|Setsteering (- _output_get_2 (Variables|Default|Getvelocity))))
    (return (Math|Vector|VectorClampSizeMax _output_get_3 (Variables|Default|GetmaxForce)))
    (else
      (return (LocalVariables|Getsteering)))))

(fn Separation
  (params (Perception%20Radius :type Float%20%28double-precision%29))
  (bind _position (Variables|Default|Getposition))
  (bind (_outactors _returnvalue) (CallFunction|SphereCast Perception%20Radius))
  (for _array_element _outactors
    (bind _asbp_boid (Utilities|Casting|CastToBP_Boid _array_element))
    (if (and (!= self _asbp_boid) _returnvalue)
      (bind _output_get (LocalVariables|Setdiff (- _position (Variables|BP_Boid_C|Getposition _asbp_boid))))
      (LocalVariables|Setsteering (+ (Math|Vector|MakeVector (.x (LocalVariables|Getsteering)) (.y (LocalVariables|Getsteering)) 0.0) (/ _output_get (Math|Vector|Distance(Vector) _position (Variables|BP_Boid_C|Getposition _asbp_boid)))))
      (Math|Integer|IncrementInt (LocalVariables|Gettotal))))
  (if (> (LocalVariables|Gettotal) 0)
    (bind _output_get_2 (LocalVariables|Setsteering (/ (LocalVariables|Getsteering) (LocalVariables|Gettotal))))
    (bind _output_get_3 (LocalVariables|Setsteering (- (* (Math|Vector|Normalize _output_get_2) (Variables|Default|GetmaxSpeed)) (Variables|Default|Getvelocity))))
    (return (Math|Vector|VectorClampSizeMax _output_get_3 (Variables|Default|GetmaxForce)))
    (else
      (return (LocalVariables|Getsteering)))))

(fn Arriving
  ;[1 1 1] Setting the desired vector
  (bind _output_get (LocalVariables|Setdesired (- "" (Variables|Default|Getposition))))
  (if (< (Math|Vector|VectorLength _output_get) 1e+02)
    (bind _output_get_2 (LocalVariables|Setm (Math|Float|MapRangeUnclamped (Math|Vector|VectorLength _output_get) 0.0 1e+02 0.0 (Variables|Default|GetmaxSpeed))))
    (LocalVariables|Setdesired (* (Math|Vector|Normalize _output_get) _output_get_2))
    (else
      (LocalVariables|Setdesired (* (Math|Vector|Normalize _output_get) (Variables|Default|GetmaxSpeed)))))
  (bind _output_get_3 (LocalVariables|Setsteering (- (LocalVariables|Getdesired) (Variables|Default|Getvelocity))))
  (return (Math|Vector|VectorClampSizeMax _output_get_3 (Variables|Default|GetmaxForce))))

(fn Fleeing
  (params (Player :type BP%20First%20Person%20Character%20Object%20Reference))
  ;[1 1 1] Setting the desired vector
  (bind _output_get (LocalVariables|Setdesired (- (Transformation|GetWorldLocation (Variables|/Game/FirstPerson/Blueprints/BP_FirstPersonCharacter.BP_FirstPersonCharacter_C|GetFirstPersonMesh Player)) (Variables|Default|Getposition))))
  (bind _output_get_2 (LocalVariables|Setdesired (* (Math|Vector|Normalize (* _output_get -1)) (Variables|Default|GetmaxSpeed))))
  (bind _output_get_3 (LocalVariables|Setsteering (- _output_get_2 (Variables|Default|Getvelocity))))
  (Variables|Default|Setacceleration (+ (Variables|Default|Getacceleration) (Math|Vector|VectorClampSizeMax _output_get_3 (Variables|Default|GetmaxForce)))))

(fn Seeking
  ;[1 1 1] Setting the desired vector
  (bind _output_get (LocalVariables|Setdesired (- "" (Variables|Default|Getposition))))
  (bind _output_get_2 (LocalVariables|Setdesired (* (Math|Vector|Normalize _output_get) (Variables|Default|GetmaxSpeed))))
  (bind _output_get_3 (LocalVariables|Setsteering (- _output_get_2 (Variables|Default|Getvelocity))))
  (return (Math|Vector|VectorClampSizeMax _output_get_3 (Variables|Default|GetmaxForce))))

(fn AvoidObstacle
  (bind _outhit (Collision|LineTraceForObjects (Variables|Default|Getposition) (+ (Variables|Default|Getposition) (* (Math|Vector|GetForwardVector (Variables|Default|GetCube)) -3.0)) (LocalVariables|GetObject) false 0 (Variables|Default|GetDraw%20Debug%20Type) true "(R=1.000000,G=0.000000,B=0.000000,A=1.000000)" "(R=1.000000,G=0.000000,B=0.097957,A=1.000000)"))
  (bind _output_get (LocalVariables|Setright%20vector (Math|Vector|GetRightVector (Variables|Default|GetCube))))
  (LocalVariables|Setleft%20vector (* (Math|Vector|GetRightVector (Variables|Default|GetCube)) -1.0))
  (Variables|Default|Setacceleration (+ (Variables|Default|Getacceleration) (+ _output_get (.ImpactPoint (Collision|BreakHitResult _outhit))))))

(fn SphereCast
  (params (PerceptionRadius :type Float%20%28double-precision%29))
  ;[1 1 1] Casting a sphere to get the amount of boids within the perception raidus
  (bind (_outactors _returnvalue) (Collision|SphereOverlapActors (Variables|Default|Getposition) PerceptionRadius (Variables|Default|GetObject%20Types) 0))
  (return _outactors _returnvalue))