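; Enemy spawner that creates BP_EnemyBase_Test enemies at random points inside its SpawnArea box whenever something begins overlapping it.
; Each overlap halves SpawnAmount, then spawns that many enemies, with an explosion effect at a separately randomized point for each.
; The first three enemies take SetElement1 and the rest SetElement2, copied to each enemy's head before its colour updates.
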(event OnComponentBeginOverlap(SpawnArea)
  (params (OverlappedComponent :type Primitive%20Component%20Object%20Reference) (OtherActor :type Actor%20Object%20Reference) (OtherComp :type Primitive%20Component%20Object%20Reference) (OtherBodyIndex :type Integer) (bFromSweep :type Boolean) (SweepResult :type Hit%20Result%20Structure%20%28by%20ref%29))
  (bind _spawn_area (Variables|Default|GetSpawn%20Area))
  (bind _spawn_area_2 (Variables|Default|GetSpawn%20Area))
  (bind _returnvalue (Transformation|GetWorldLocation _spawn_area_2))
  (bind _returnvalue_2 (Components|Box|GetScaledBoxExtent _spawn_area))
  (bind _returnvalue_3 (Math|Random|RandomPointinBoundingBox _returnvalue _returnvalue_2))
  (Variables|Default|SetSpawnAmount (/ (Variables|Default|GetSpawnAmount) 2))
  (for _index (range 1 (Variables|Default|GetSpawnAmount))
    (Effects|SpawnEmitteratLocation "/Game/StarterContent/Particles/P_Explosion.P_Explosion" _returnvalue_3)
    (bind _returnvalue_4 (Game|SpawnActorfromClass "/Game/Enemies/Blueprints/Test/BP_EnemyBase_Test.BP_EnemyBase_Test_C" (Math|Conversions|ToTransform(Vector) _returnvalue_3) "Undefined" 0 0))
    (if (> _index 3)
      (bind _output_get (Variables|/Game/Enemies/Blueprints/BP_EnemyBase.BP_EnemyBase_C|SetElement _returnvalue_4 (Variables|Default|GetSet%20Element%202)))
      (Variables|/Game/Enemies/Blueprints/BP_EnemyHeadBase.BP_EnemyHeadBase_C|SetElement (Variables|/Game/Enemies/Blueprints/BP_EnemyBase.BP_EnemyBase_C|GetEnemy%20Head%20REF _returnvalue_4) _output_get)
      (else
        (bind _output_get_2 (Variables|/Game/Enemies/Blueprints/BP_EnemyBase.BP_EnemyBase_C|SetElement _returnvalue_4 (Variables|Default|GetSet%20Element%201)))
        (Variables|/Game/Enemies/Blueprints/BP_EnemyHeadBase.BP_EnemyHeadBase_C|SetElement (Variables|/Game/Enemies/Blueprints/BP_EnemyBase.BP_EnemyBase_C|GetEnemy%20Head%20REF _returnvalue_4) _output_get_2)))
    (Default|ChangeColour (Variables|/Game/Enemies/Blueprints/BP_EnemyBase.BP_EnemyBase_C|GetEnemy%20Head%20REF _returnvalue_4))))

(event EventBeginPlay)

(fn ConstructionScript)