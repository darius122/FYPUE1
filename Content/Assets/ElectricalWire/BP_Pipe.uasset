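; BP_Pipe is an actor that builds a pipe along an editable spline.
; Its construction script divides the spline into SplineLength segments, adding a spline mesh component with the assigned Material for each full segment and leaving any shorter remainder uncovered.
; Segment ends and tangents are sampled in local space, with tangents clamped to segment length.
; The event graph has no active logic.
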(event EventBeginPlay)

(event Collision|EventActorBeginOverlap
  (params (OtherActor :type Actor%20Object%20Reference)))

(event EventTick
  (params (DeltaSeconds :type Float%20%28single-precision%29)))

(fn ConstructionScript
  (bind _spline (Variables|Default|GetSpline))
  (bind _spline_length (Variables|Default|GetSpline%20Length))
  (bind _spline_length_2 (Variables|Default|GetSpline%20Length))
  (for _index (range 0 (Math|Float|Truncate (/ (Spline|GetSplineLength (Variables|Default|GetSpline)) (Variables|Default|GetSpline%20Length))))
    (if (not (> (+ (* _index _spline_length) _spline_length) (Spline|GetSplineLength (Variables|Default|GetSpline))))
      (bind _returnvalue (AddComponent|AddSplineMeshComponent false))
      (Rendering|Material|SetMaterial _returnvalue 0 (Variables|Default|GetMaterial))
      (SplineMesh|SetStartandEnd _returnvalue (Spline|GetLocationatDistanceAlongSpline _spline (* _index _spline_length) "Local") (Math|Vector|ClampVectorSize (Spline|GetTangentatDistanceAlongSpline _spline (* _index _spline_length) "Local") 0.0 _spline_length_2) (Spline|GetLocationatDistanceAlongSpline _spline (+ (* _index _spline_length) _spline_length) "Local") (Math|Vector|ClampVectorSize (Spline|GetTangentatDistanceAlongSpline _spline (+ (* _index _spline_length) _spline_length) "Local") 0.0 _spline_length_2) true :!class /Script/Engine.SplineMeshComponent))))