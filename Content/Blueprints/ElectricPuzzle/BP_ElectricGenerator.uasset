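; Electric generator actor for the electric puzzle, with an emissive glow on its Cube and a link to a dissolvable door.
; The glow starts at zero, and SetEmissionValue animates it through the Emission timeline's curve.
; ResetEmissionValue reverses a separate timeline whose updates force the glow to zero rather than fading it.
; DissolveDoor forwards the call to the referenced Door when it is valid.
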(event Custom|Set%20EmissionValue
  (bind _newtrack_0 (Timeline|Emission Play)
    (:Update
      (Rendering|Material|SetScalarParameterValueonMaterials (Variables|Default|GetCube) "Emissive Strength" _newtrack_0))))

(event Custom|Reset%20EmissionValue
  (Timeline|Timeline Reverse
    (:Update
      (Rendering|Material|SetScalarParameterValueonMaterials (Variables|Default|GetCube) "Emissive Strength" 0.0))))

(event Custom|DissolveDoor
  (bind _door (Variables|Default|GetDoor))
  (Utilities|IsValid _door
    (:Is%20Valid
      (Default|DissolveDoor _door))))

(event EventBeginPlay
  (Rendering|Material|SetScalarParameterValueonMaterials (Variables|Default|GetCube) "Emissive Strength" 0.0))

(event Collision|EventActorBeginOverlap
  (params (OtherActor :type Actor%20Object%20Reference)))

(event EventTick
  (params (DeltaSeconds :type Float%20%28single-precision%29)))

(fn ConstructionScript)