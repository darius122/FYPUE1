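; Game manager that polls the level's puzzles every Tick while Run is set and dissolves a door once PassElectric and PassTrain are true.
; Light puzzle tracks the reflector hit by the light source and switches off reflector lasers when the hit is lost.
; Generator puzzle records activation order, compares it to SequenceArray and resets on a mismatch.
; Connected wagons mirror the train's start state; PassTrain is only read here.
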(event EventBeginPlay
  (bind _asbp_first_person_character (Utilities|Casting|CastToBP_FirstPersonCharacter (Pawn|GetControlledPawn (Game|GetPlayerController 0))))
  (Variables|Default|SetPlayerREF _asbp_first_person_character))

(event Collision|EventActorBeginOverlap
  (params (OtherActor :type Actor%20Object%20Reference)))

(event EventTick
  (params (DeltaSeconds :type Float%20%28single-precision%29))
  (bind _lightsource (Variables|Default|GetLightSource))
  (bind _door (Variables|Default|GetDoor))
  (bind _lightsourcehitactorref (Variables|/Game/Blueprints/LightPuzzle/BP_ReflectorLocation.BP_ReflectorLocation_C|GetLightSourceHitActorREF _lightsource))
  (if (Variables|Default|GetRun)
    (Utilities|FlowControl|Sequence
      (:then_0
        ;[1 1 1] Light Reflector Puzzle
        (for _array_element (Variables|Default|GetItemLocArray)
          (Variables|Default|SetArray%20Element _array_element)
          ;;[1 1 1] Checks if Light Source is hitting a reflector
          (if (Utilities|IsValid _lightsourcehitactorref)
            ;;[1 1 1] Check if the array element is equal to the actor the light source hits
            (if (== _lightsourcehitactorref _array_element)
              (Variables|Default|Setinitial%20hit (Variables|Default|GetArray%20Element)))
            (else
              ;;[1 1 1] If False, check if the Initial Hit Object is Valid and then setting the IsHitByLight bool of it to false
              (Utilities|IsValid (Variables|Default|Getinitial%20hit)
                (:Is%20Valid
                  (Variables|/Game/Blueprints/LightPuzzle/BP_ReflectorLocation.BP_ReflectorLocation_C|SetisCastingRay? (Variables|Default|GetArray%20Element) false)
                  (Variables|/Game/Blueprints/LightPuzzle/BP_ReflectorLocation.BP_ReflectorLocation_C|SetLight%20Range (Variables|Default|GetArray%20Element) 0.0)
                  (Rendering|SetVisibility (Variables|/Game/Blueprints/LightPuzzle/BP_ReflectorLocation.BP_ReflectorLocation_C|GetNiagaraLaser (Variables|Default|GetArray%20Element)) false false)))))))
      (:then_1
        ;[1 1 1] Sequencing Puzzle
        (for _array_element_2 (Variables|Default|GetGeneratorArray)
          (if (Math|Conversions|ToBoolean(Integer) (Class|KismetMathLibrary|AndIntInt (Math|Conversions|ToInteger(Boolean) (Variables|/Game/Blueprints/ElectricPuzzle/BP_ElectricGenerator.BP_ElectricGenerator_C|GetisActivated? _array_element_2)) (Math|Conversions|ToInteger(Boolean) (== (Variables|/Game/Blueprints/ElectricPuzzle/BP_ElectricGenerator.BP_ElectricGenerator_C|GetisNumAdded? _array_element_2) false))))
            (Utilities|Array|Add (Variables|Default|GetNumOrderArray) (Variables|/Game/Blueprints/ElectricPuzzle/BP_ElectricGenerator.BP_ElectricGenerator_C|GetOrderIndex _array_element_2))
            (Variables|/Game/Blueprints/ElectricPuzzle/BP_ElectricGenerator.BP_ElectricGenerator_C|SetisNumAdded? _array_element_2 true)))
        (if (Math|Conversions|ToBoolean(Integer) (Class|KismetMathLibrary|AndIntInt (Math|Conversions|ToInteger(Boolean) (== (Utilities|Array|Length (Variables|Default|GetNumOrderArray)) (Utilities|Array|Length (Variables|Default|GetGeneratorArray)))) (Math|Conversions|ToInteger(Boolean) (Variables|Default|GetisInOrder))))
          (for (_array_element_3 _array_index) (Variables|Default|GetNumOrderArray)
            (if (== _array_element_3 (Utilities|Array|Get(acopy) (Variables|Default|GetSequenceArray) _array_index))
              (Variables|Default|SetPassElectric true)
              (else
                (Variables|Default|SetisInOrder false)
                (Variables|Default|SetPassElectric false)
                (Utilities|Array|Clear (Variables|Default|GetNumOrderArray))
                (for _array_element_4 (Variables|Default|GetGeneratorArray)
                  (Variables|/Game/Blueprints/ElectricPuzzle/BP_ElectricGenerator.BP_ElectricGenerator_C|SetisActivated? _array_element_4 false)
                  (Variables|/Game/Blueprints/ElectricPuzzle/BP_ElectricGenerator.BP_ElectricGenerator_C|SetisNumAdded? _array_element_4 false)
                  (Variables|Default|SetisInOrder true)
                  (Utilities|FlowControl|Delay 3.0)
                  (Default|ResetLight (Variables|Default|GetPowerBox))))))))
      (:then_2
        ;[1 1 1] Train
        (if (Variables|/Game/Blueprints/Train/BP_Train.BP_Train_C|GetisStart? (Variables|Default|GetTrain))
          (for _array_element_5 (Variables|Default|GetWagons)
            (if (Variables|/Game/Blueprints/Train/BP_Train.BP_Train_C|GetIsConnected? _array_element_5)
              (Variables|/Game/Blueprints/Train/BP_Train.BP_Train_C|SetisStart? _array_element_5 true)))
          (else
            (for _array_element_6 (Variables|Default|GetWagons)
              (if (Variables|/Game/Blueprints/Train/BP_Train.BP_Train_C|GetIsConnected? _array_element_6)
                (Variables|/Game/Blueprints/Train/BP_Train.BP_Train_C|SetisStart? _array_element_6 false))))))
      (:then_3
        (if (Math|Conversions|ToBoolean(Integer) (Class|KismetMathLibrary|AndIntInt (Math|Conversions|ToInteger(Boolean) (Variables|Default|GetPassElectric)) (Math|Conversions|ToInteger(Boolean) (Variables|Default|GetPassTrain))))
          (Utilities|IsValid _door
            (:Is%20Valid
              (Default|DissolveDoor _door))))))))

(fn ConstructionScript)