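; BP_RotatorPanel is a panel actor with a widget component that rotates a referenced RotatingTrack actor clockwise or anticlockwise.
; Two custom events, one per direction, each restart a timeline that eases the track's root world rotation toward that direction's target rotator.
; Each update uses RInterpTo, with the timeline track value fed in as DeltaTime.
; BeginPlay caches the widget's world location, which these graphs do not use further.
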(event Custom|RotateClockwise_Event
  (bind _rotating_track (Variables|Default|GetRotating%20Track))
  (bind _rootcomponent (Variables|/Script/Engine.Actor|GetRootComponent _rotating_track))
  (bind _newtrack_1 (Timeline|Timeline PlayFromStart)
    (:Update
      (Transformation|SetWorldRotation _rootcomponent (Math|Interpolation|RInterpTo (Transformation|GetWorldRotation _rootcomponent) (Variables|Default|GetClockWiseRotator) _newtrack_1 0.2) false false))))

(event Custom|RotateAnitClockwise_Event
  (bind _rotating_track (Variables|Default|GetRotating%20Track))
  (bind _rootcomponent (Variables|/Script/Engine.Actor|GetRootComponent _rotating_track))
  (bind _newtrack_1 (Timeline|Timeline_0 PlayFromStart)
    (:Update
      (Transformation|SetWorldRotation _rootcomponent (Math|Interpolation|RInterpTo (Transformation|GetWorldRotation _rootcomponent) (Variables|Default|GetAntiClockWiseRotator) _newtrack_1 0.2) false false))))

(event EventBeginPlay
  (Variables|Default|SetWidget%20loc (Transformation|GetWorldLocation (Variables|Default|GetWidget))))

(event Collision|EventActorBeginOverlap
  (params (OtherActor :type Actor%20Object%20Reference)))

(event EventTick
  (params (DeltaSeconds :type Float%20%28single-precision%29)))

(fn ConstructionScript)