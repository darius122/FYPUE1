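; BP_GameManager is a manager Blueprint that opens the first section by removing its wall once that section's key is gone.
; Tick polls Section1Key until it is no longer valid, then destroys Section1Wall and sets Section1Done so this runs only once.
; A check for four destroyed Section1Boxes is left unconnected, despite the Tick comment describing that condition.
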(event EventBeginPlay)

(event Collision|EventActorBeginOverlap
  (params (OtherActor :type Actor%20Object%20Reference)))

(event EventTick
  (params (DeltaSeconds :type Float%20%28single-precision%29))
  ;[0 0 0] Check if All Boxes are Destoryed
  (if (not (Variables|Default|GetSection%201%20Done))
    (if (== (Utilities|IsValid (Variables|Default|GetSection%201%20Key)) false)
      (Actor|DestroyActor (Variables|Default|GetSection%201%20Wall))
      (Variables|Default|SetSection%201%20Done true))))

(fn ConstructionScript)