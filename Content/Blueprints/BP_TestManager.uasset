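; Manager Blueprint that tracks which reflector the light source hits and shuts off reflector beams when that hit is lost.
; Each Tick it loops ItemLocArray, storing the element matching LightSourceHitActorREF as InitialHit.
; With no valid hit but a valid InitialHit, it stops every element's ray casting, zeroes its light range and hides its Niagara laser.
; InitialHit is never cleared, so that shutdown repeats each frame.
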(event EventBeginPlay)

(event Collision|EventActorBeginOverlap
  (params (OtherActor :type Actor%20Object%20Reference)))

(event EventTick
  (params (DeltaSeconds :type Float%20%28single-precision%29))
  (bind _lightsource (Variables|Default|GetLightSource))
  (bind _lightsourcehitactorref (Variables|/Game/Blueprints/BP_ReflectorLocation.BP_ReflectorLocation_C|GetLightSourceHitActorREF _lightsource))
  (for _array_element (Variables|Default|GetItemLocArray)
    ;[1 1 1] Checks if Light Source is hitting a reflector
    (if (Utilities|IsValid _lightsourcehitactorref)
      ;[1 1 1] Check if the array element is equal to the actor the light source hits
      (if (== _lightsourcehitactorref _array_element)
        (bind _output_get (Variables|Default|Setinitial%20hit _array_element)))
      (else
        ;[1 1 1] If False, check if the Initial Hit Object is Valid and then setting the IsHitByLight bool of it to false
        (Utilities|IsValid _output_get
          (:Is%20Valid
            (Variables|/Game/Blueprints/BP_ReflectorLocation.BP_ReflectorLocation_C|SetisCastingRay? _array_element false)
            (Variables|/Game/Blueprints/BP_ReflectorLocation.BP_ReflectorLocation_C|SetLight%20Range _array_element 0.0)
            (Rendering|SetVisibility (Variables|/Game/Blueprints/BP_ReflectorLocation.BP_ReflectorLocation_C|GetNiagaraLaser _array_element) false false)))))))

(fn ConstructionScript)