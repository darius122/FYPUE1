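; BP_Pipe is a spline-driven pipe actor that builds its geometry in the construction script, with no active runtime logic.
; It walks the spline in fixed 800-unit steps, adding one spline mesh component per full segment and skipping any shorter remainder at the end.
; Each segment takes its local-space endpoints and tangents from the spline, with tangent length clamped to the segment length so consecutive pieces bend cleanly along the curve.
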(event EventBeginPlay)

(event Collision|EventActorBeginOverlap
  (params (OtherActor :type Actor%20Object%20Reference)))

(event EventTick
  (params (DeltaSeconds :type Float%20%28single-precision%29)))

(fn ConstructionScript
  (bind _spline (Variables|Default|GetSpline))
  (bind _spline_2 (Variables|Default|GetSpline))
  (for _index (range 0 (Math|Float|Truncate (/ (Spline|GetSplineLength (Variables|Default|GetSpline)) 8e+02)))
    (if (not (> (+ (* _index 8e+02) 8e+02) (Spline|GetSplineLength (Variables|Default|GetSpline))))
      (bind _returnvalue (AddComponent|AddSplineMeshComponent false))
      (SplineMesh|SetStartandEnd _returnvalue (Spline|GetLocationatDistanceAlongSpline _spline_2 (* _index 8e+02) "Local") (Math|Vector|ClampVectorSize (Spline|GetTangentatDistanceAlongSpline _spline_2 (* _index 8e+02) "Local") 0.0 8e+02) (Spline|GetLocationatDistanceAlongSpline _spline (+ (* _index 8e+02) 8e+02) "Local") (Math|Vector|ClampVectorSize (Spline|GetTangentatDistanceAlongSpline _spline (+ (* _index 8e+02) 8e+02) "Local") 0.0 8e+02) true :!class /Script/Engine.SplineMeshComponent))))