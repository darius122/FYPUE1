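; BP_ItemLocation is a light-puzzle socket where a nearby player presses F to place one of three matching items, revealing its LightCaster.
; Each Tick, a debug-drawn sphere overlap finds the player, whose Q/E keys pitch, yaw or slide the socket along Y, depending on the item.
; Sources and lit sockets line-trace light, flagging other sockets to relay it; the flag resets every Tick.
; Hitting BP_LightTarget only prints a message.
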(event EventBeginPlay)

(event Collision|EventActorBeginOverlap
  (params (OtherActor :type Actor%20Object%20Reference)))

(event EventTick
  (params (DeltaSeconds :type Float%20%28single-precision%29))
  (CallFunction|CheckPlayer)
  (CallFunction|CheckItemAttached)
  (Variables|Default|SetisHitbyLight false))

(fn ConstructionScript)

(fn CheckPlayer
  (bind _returnvalue (Game|GetPlayerController 0))
  (bind _returnvalue_2 (Game|GetPlayerController 0))
  (bind _cube (Variables|Default|GetCube))
  (bind _defaultsceneroot (Variables|Default|GetDefaultSceneRoot))
  (bind _returnvalue_3 (Transformation|GetWorldLocation _cube))
  (bind _returnvalue_4 (Game|Player|IsInputKeyDown _returnvalue "F"))
  (bind _returnvalue_5 (Game|Player|IsInputKeyDown _returnvalue_2 "Q"))
  (bind _returnvalue_6 (Transformation|GetWorldLocation _defaultsceneroot))
  (bind _returnvalue_7 (Game|Player|IsInputKeyDown _returnvalue_2 "E"))
  (bind _returnvalue_8 (Math|Conversions|ToInteger(Boolean) _returnvalue_4))
  ;[1 1 1] Check if Player is in radius of object
  (Rendering|Debug|DrawDebugSphere _returnvalue_3 2e+02 12 "(R=1.000000,G=1.000000,B=1.000000,A=1.000000)" 0.0)
  (bind _outactors (Collision|SphereOverlapActors _returnvalue_3 2e+02 (Variables|Default|GetObject%20Types) 0))
  (for _array_element _outactors
    (bind _asbp_first_person_character (Utilities|Casting|CastToBP_FirstPersonCharacter _array_element))
    (Utilities|FlowControl|Sequence
      (:then_0
        (if (Math|Conversions|ToBoolean(Integer) (Class|KismetMathLibrary|AndIntInt (Class|KismetMathLibrary|AndIntInt (Math|Conversions|ToInteger(Boolean) (Variables|/Game/FirstPerson/Blueprints/BP_FirstPersonCharacter.BP_FirstPersonCharacter_C|GetIsHavingItem1 _asbp_first_person_character)) _returnvalue_8) (Math|Conversions|ToInteger(Boolean) (Utilities|Enum|Equal(Enum) (Variables|Default|GetItem) (Utilities|Enum|LiteralenumItems "NewEnumerator0")))))
          (Variables|/Game/FirstPerson/Blueprints/BP_FirstPersonCharacter.BP_FirstPersonCharacter_C|SetIsHavingItem1 _asbp_first_person_character false)
          (Rendering|SetVisibility (Variables|Default|GetLight%20Caster) true false)
          (Variables|Default|SetisItem1Attached? true)
          (elif (Math|Conversions|ToBoolean(Integer) (Class|KismetMathLibrary|AndIntInt (Class|KismetMathLibrary|AndIntInt (Math|Conversions|ToInteger(Boolean) (Variables|/Game/FirstPerson/Blueprints/BP_FirstPersonCharacter.BP_FirstPersonCharacter_C|GetIsHavingItem2 _asbp_first_person_character)) _returnvalue_8) (Math|Conversions|ToInteger(Boolean) (Utilities|Enum|Equal(Enum) (Variables|Default|GetItem) (Utilities|Enum|LiteralenumItems "NewEnumerator1")))))
            (Variables|/Game/FirstPerson/Blueprints/BP_FirstPersonCharacter.BP_FirstPersonCharacter_C|SetIsHavingItem2 _asbp_first_person_character false)
            (Rendering|SetVisibility (Variables|Default|GetLight%20Caster) true false)
            (Variables|Default|SetisItem2Attached? true)
            (elif (Math|Conversions|ToBoolean(Integer) (Class|KismetMathLibrary|AndIntInt (Class|KismetMathLibrary|AndIntInt (Math|Conversions|ToInteger(Boolean) (Variables|/Game/FirstPerson/Blueprints/BP_FirstPersonCharacter.BP_FirstPersonCharacter_C|GetIsHavingItem3 _asbp_first_person_character)) _returnvalue_8) (Math|Conversions|ToInteger(Boolean) (Utilities|Enum|Equal(Enum) (Variables|Default|GetItem) (Utilities|Enum|LiteralenumItems "NewEnumerator2")))))
              (Variables|/Game/FirstPerson/Blueprints/BP_FirstPersonCharacter.BP_FirstPersonCharacter_C|SetIsHavingItem3 _asbp_first_person_character false)
              (Rendering|SetVisibility (Variables|Default|GetLight%20Caster) true false)
              (Variables|Default|SetisItem3Attached? true)))))
      (:then_1
        (if (Variables|Default|GetisItem1Attached?)
          (if _returnvalue_5
            (bind _output_get (Variables|Default|SetlightCasterYRot (+ (stale _output_get) 0.1)))
            (Transformation|SetRelativeRotation (Variables|Default|GetLight%20Caster) (Math|Rotator|MakeRotator 0.0 (Variables|Default|GetlightCasterYRot) 0.0) false false :!label _label)
            (elif _returnvalue_7
              (bind _output_get_2 (Variables|Default|SetlightCasterYRot (- (stale _output_get_2) 0.1)))
              (goto _label)))
          (elif (Variables|Default|GetisItem2Attached?)
            (if _returnvalue_5
              (bind _output_get_3 (Variables|Default|SetlightCasterZRot (+ (stale _output_get_3) 0.1)))
              (Transformation|SetRelativeRotation (Variables|Default|GetLight%20Caster) (Math|Rotator|MakeRotator 0.0 0.0 (Variables|Default|GetlightCasterZRot)) false false :!label _label_2)
              (elif _returnvalue_7
                (bind _output_get_4 (Variables|Default|SetlightCasterZRot (- (stale _output_get_4) 0.1)))
                (goto _label_2)))
            (elif (Variables|Default|GetisItem3Attached?)
              (if _returnvalue_7
                (Variables|Default|SetitemLocationYPos (.y _returnvalue_6))
                (bind _output_get_5 (Variables|Default|SetitemLocationYPos (+ (stale _output_get_5) 1.0)))
                (Transformation|SetActorLocation (Math|Vector|MakeVector (.x _returnvalue_6) (Variables|Default|GetitemLocationYPos) (.z _returnvalue_6)) true false :!label _label_3)
                (elif _returnvalue_5
                  (Variables|Default|SetitemLocationYPos (.y _returnvalue_6))
                  (bind _output_get_6 (Variables|Default|SetitemLocationYPos (- (stale _output_get_6) 1.0)))
                  (goto _label_3))))))))))

(fn CastLight
  (bind _light_caster (Variables|Default|GetLight%20Caster))
  (bind _outhit (Collision|LineTraceForObjects (Transformation|GetWorldLocation _light_caster) (* (Math|Vector|GetForwardVector (Transformation|GetWorldRotation _light_caster)) (Variables|Default|GetLight%20Range)) (Variables|Default|GetObject%20Types) false 0 "ForOneFrame" true "(R=0.028752,G=0.000000,B=1.000000,A=1.000000)" "(R=1.000000,G=0.000000,B=0.057065,A=1.000000)" 0.1))
  (Utilities|Casting|CastToBP_LightTarget (.HitActor (Collision|BreakHitResult _outhit))
    (:then
      (Development|PrintString "HIT"))
    (:CastFailed
      (bind _asbp_item_location (Utilities|Casting|CastToBP_ItemLocation (.HitActor (Collision|BreakHitResult _outhit))))
      (Variables|BP_ItemLocation_C|SetisHitbyLight _asbp_item_location true)
      (Development|PrintString "Hello"))))

(fn CheckItemAttached
  (if (Variables|Default|GetisLightSource)
    (CallFunction|CastLight)
    (elif (Variables|Default|GetisHitbyLight)
      (CallFunction|CastLight))))