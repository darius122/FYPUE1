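; BP_Train is a pawn for a train engine or wagon that rides along the BP_TrackSpline spline.
; Tick advances a spline distance by Speed, sets the Train transform and movement max speed, then loops or stops past the track ends.
; A wagon whose Front overlaps a "Back" component starts moving at that pawn's max speed.
; A ChangeLane branch follows ChangeTrackSpline, but its spline lookup and end handling are unwired.
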(event OnComponentBeginOverlap(Front)
  (params (OverlappedComponent :type Primitive%20Component%20Object%20Reference) (OtherActor :type Actor%20Object%20Reference) (OtherComp :type Primitive%20Component%20Object%20Reference) (OtherBodyIndex :type Integer) (bFromSweep :type Boolean) (SweepResult :type Hit%20Result%20Structure%20%28by%20ref%29))
  (if (Variables|Default|GetisWagon?)
    (if (Utilities|Enum|Equal(Enum) (Utilities|GetObjectName OtherComp) "Back")
      (bind _aspawn (Utilities|Casting|CastToPawn OtherActor))
      (Variables|Default|SetisStart? true)
      (Variables|Default|SetSpeed (Class|MovementComponent|GetMaxSpeed (Pawn|GetMovementComponent _aspawn))))))

(event EventBeginPlay
  (bind _returnvalue (Actor|GetActorOfClass "/Game/Blueprints/BP_TrackSpline.BP_TrackSpline_C"))
  (Variables|Default|SetTrack%20Spline (Variables|/Game/Blueprints/BP_TrackSpline.BP_TrackSpline_C|GetTrackSpline _returnvalue))
  ;[1 1 1] Get Position of Train Relative to the Spline Distance
  (Variables|Default|SetTrain%20Distance (Class|SplineComponent|GetDistanceAlongSplineatSplineInputKey (Variables|Default|GetTrack%20Spline) (Class|SplineComponent|FindInputKeyClosesttoWorldLocation (Variables|Default|GetTrack%20Spline) (Transformation|GetWorldLocation (Variables|Default|GetTrain))))))

(event Collision|EventActorBeginOverlap
  (params (OtherActor :type Actor%20Object%20Reference)))

(event EventTick
  (params (DeltaSeconds :type Float%20%28single-precision%29))
  (if (Variables|Default|GetisStart?)
    (Variables|Default|SetTrain%20Distance (+ (Variables|Default|GetTrain%20Distance) (* DeltaSeconds (Variables|Default|GetSpeed))))
    (if (Variables|Default|GetChangeLane?)
      ;[1 1 1] Move Train
      (Transformation|SetWorldTransform (Variables|Default|GetTrain) (Math|Transform|MakeTransform (.location (Spline|GetTransformatDistanceAlongSpline (Variables|Default|GetChange%20Track%20Spline) (Variables|Default|GetTrain%20Distance) "World" false)) (.rotation (Spline|GetTransformatDistanceAlongSpline (Variables|Default|GetChange%20Track%20Spline) (Variables|Default|GetTrain%20Distance) "World" false)) "1.000000,1.000000,1.000000") false false)
      ;[1 1 1] Set Max Speed of Pawn
      (Variables|/Script/Engine.FloatingPawnMovement|SetMaxSpeed (Variables|Default|GetFloatingPawnMovement) (Variables|Default|GetSpeed))
      (else
        ;[1 1 1] Move Train
        (Transformation|SetWorldTransform (Variables|Default|GetTrain) (Math|Transform|MakeTransform (.location (Spline|GetTransformatDistanceAlongSpline (Variables|Default|GetTrack%20Spline) (Variables|Default|GetTrain%20Distance) "World" false)) (.rotation (Spline|GetTransformatDistanceAlongSpline (Variables|Default|GetTrack%20Spline) (Variables|Default|GetTrain%20Distance) "World" false)) "1.000000,1.000000,1.000000") false false)
        ;[1 1 1] Set Max Speed of Pawn
        (Variables|/Script/Engine.FloatingPawnMovement|SetMaxSpeed (Variables|Default|GetFloatingPawnMovement) (Variables|Default|GetSpeed))
        ;[1 1 1] Loop Train
        (if (>= (Variables|Default|GetTrain%20Distance) (Spline|GetSplineLength (Variables|Default|GetTrack%20Spline)))
          (Variables|Default|SetCalc%20Distance 0.0)
          (if (Variables|Default|GetisLoop?) :!label _label
            (Variables|Default|SetTrain%20Distance (Variables|Default|GetCalc%20Distance))
            (else
              (Variables|Default|SetSpeed 0.0)
              (Variables|Default|SetisStart? false)))
          (elif (< (Variables|Default|GetTrain%20Distance) 0.0)
            (Variables|Default|SetCalc%20Distance (- (Spline|GetSplineLength (Variables|Default|GetTrack%20Spline)) (Variables|Default|GetTrain%20Distance)))
            (goto _label)))))))

(fn ConstructionScript)