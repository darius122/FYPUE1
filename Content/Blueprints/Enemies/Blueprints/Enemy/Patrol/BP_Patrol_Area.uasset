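; Patrol area actor that groups the BP_Patrol_Point actors inside its bounds into a looping route for enemy patrols.
; On BeginPlay it scans all patrol points, keeps those in range and numbers them in the order found.
; The range test is an axis-aligned X/Y box derived from actor scale at 100 units each, ignoring height and rotation.
; GetNextPoint returns the following point, wrapping to the first after the last.
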(event EventBeginPlay
  ;[1 1 1] All Points
  (bind _outactors (Actor|GetAllActorsOfClass "/Game/Blueprints/Enemies/Blueprints/Enemy/Patrol/BP_Patrol_Point.BP_Patrol_Point_C"))
  ;[1 1 1] Check in range and register
  (for _array_element _outactors
    (if (CallFunction|CheckinRange (Transformation|GetActorLocation _array_element))
      (Utilities|Array|Add (Variables|Default|GetPatrol%20Point%20List) _array_element)
      (for (_array_element_2 _array_index) (Variables|Default|GetPatrol%20Point%20List)
        (Variables|/Game/Blueprints/Enemies/Blueprints/Enemy/Patrol/BP_Patrol_Point.BP_Patrol_Point_C|SetNumber _array_element_2 _array_index))
      (Variables|Default|SetAll%20Points%20Number (Utilities|Array|Length (Variables|Default|GetPatrol%20Point%20List))))))

(fn ConstructionScript)

(fn GetNextPointNumber
  (params (Now%20Point :type Integer))
  (if (>= Now%20Point (- (Variables|Default|GetAll%20Points%20Number) 1))
    (return 0)
    (else
      (return (+ Now%20Point 1)))))

(fn GetNextPoint
  (params (Now%20Point :type Integer))
  (return (Utilities|Array|Get(acopy) (Variables|Default|GetPatrol%20Point%20List) (CallFunction|GetNextPointNumber Now%20Point))))

(fn AxisCheckinRange
  (params (Point%20Axis :type Float%20%28double-precision%29) (Area%20Axis%20Center :type Float%20%28double-precision%29) (Axis%20Scale :type Float%20%28double-precision%29))
  (bind _returnvalue (* Axis%20Scale 0.5))
  (bind _returnvalue_2 (* _returnvalue 1e+02))
  (return (and (<= (+ Area%20Axis%20Center (* _returnvalue_2 -1.0)) Point%20Axis) (<= Point%20Axis (+ Area%20Axis%20Center _returnvalue_2)))))

(fn CheckinRange
  (params (Point%20Location :type Vector))
  (bind _returnvalue (Transformation|GetActorLocation))
  (bind _returnvalue_2 (Transformation|GetActorScale3D))
  (return (Math|Boolean|ANDBoolean (CallFunction|AxisCheckinRange (.x Point%20Location) (.x _returnvalue) (.x _returnvalue_2)) (CallFunction|AxisCheckinRange (.y Point%20Location) (.y _returnvalue) (.y _returnvalue_2)) true)))