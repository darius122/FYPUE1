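; Test electric enemy variant that extends its parent enemy's BeginPlay to set up an electric head, health and colors.
; It spawns a BP_EnemyHeadElectric and snaps it to the mesh's head socket, then raises max health by HeadCount, refills health and sets two yellow tint colors.
; It also snaps a melee hammer to the right wrist socket.
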(event EventBeginPlay
  (|CallParentFunction)
  (Utilities|FlowControl|Sequence
    (:then_0
      (bind _returnvalue (Game|SpawnActorfromClass "/Game/Blueprints/Enemies/Blueprints/EnemyHead/BP_EnemyHeadElectric.BP_EnemyHeadElectric_C" (Transformation|GetSocketTransform (Variables|Character|GetMesh) "Head_jntSocket" "RTS_World") "Undefined" 0 0))
      (Transformation|AttachComponentToComponent _returnvalue (Variables|Character|GetMesh) "Head_jntSocket" "SnapToTarget" "SnapToTarget" "SnapToTarget" true)
      (bind _output_get (Variables|Default|SetEnemyMaxHealth (+ (Variables|Default|GetEnemyMaxHealth) (* 10 (Variables|Default|GetHeadCount)))))
      (Variables|Default|SetEnemyHealth _output_get)
      (Variables|Default|SetColor1 "(R=1.000000,G=0.698233,B=0.000000,A=1.000000)")
      (Variables|Default|SetColor2 "(R=0.614583,G=0.507694,B=0.065921,A=1.000000)"))
    (:then_1
      (Transformation|AttachComponentToComponent (Variables|Default|GetEE_MeleeAttack_Anim_nohead_Hammer) (Variables|Character|GetMesh) "R_Wrist_jntSocket" "SnapToTarget" "SnapToTarget" "SnapToTarget" true))))

(event Collision|EventActorBeginOverlap
  (params (OtherActor :type Actor%20Object%20Reference)))

(event EventTick
  (params (DeltaSeconds :type Float%20%28single-precision%29))
  (|CallParentFunction DeltaSeconds) ; This node is disabled and will not be called.\nDrag off pins to build functionality.
)

(fn ConstructionScript
  (|CallParentFunction))