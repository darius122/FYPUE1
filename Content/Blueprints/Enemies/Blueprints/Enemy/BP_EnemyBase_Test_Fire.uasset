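; A fire variant of an enemy, apparently a test asset, that layers fire-specific setup on its parent class's BeginPlay.
; It spawns a fire head actor and snaps it to the mesh's head socket, then adds a HeadCount-scaled bonus to max health, refills current health and sets two red-toned colors.
; It also attaches a crossbrace component to a right middle-finger socket.
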(event EventBeginPlay
  (|CallParentFunction)
  (Utilities|FlowControl|Sequence
    (:then_0
      (bind _returnvalue (Game|SpawnActorfromClass "/Game/Blueprints/Enemies/Blueprints/EnemyHead/BP_EnemyHeadFire.BP_EnemyHeadFire_C" (Transformation|GetSocketTransform (Variables|Character|GetMesh) "Head_jntSocket" "RTS_World") "AlwaysSpawn" 0 0))
      (Transformation|AttachComponentToComponent _returnvalue (Variables|Character|GetMesh) "Head_jntSocket" "SnapToTarget" "SnapToTarget" "SnapToTarget" true)
      (bind _output_get (Variables|Default|SetEnemyMaxHealth (+ (Variables|Default|GetEnemyMaxHealth) (* 10 (Variables|Default|GetHeadCount)))))
      (Variables|Default|SetEnemyHealth _output_get)
      (Variables|Default|SetColor1 "(R=1.000000,G=0.009362,B=0.000000,A=1.000000)")
      (Variables|Default|SetColor2 "(R=0.614583,G=0.083186,B=0.089300,A=1.000000)"))
    (:then_1
      (Transformation|AttachComponentToComponent (Variables|Default|GetFE_WalkAnim_body_Crossbrace) (Variables|Character|GetMesh) "R_MiddleF_jnt1Socket" "SnapToTarget" "SnapToTarget" "SnapToTarget" true))))

(fn ConstructionScript
  (|CallParentFunction))