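; BP_TestEnemy1 is a test enemy pawn that flags in its AI blackboard when it has spotted the player.
; PawnSensing's OnSeePawn filters for BP_FirstPersonCharacter and sets the hasSeenPlayer key to true.
; A 0.6-second retriggerable delay then clears the key, so the flag holds while sightings repeat and drops shortly after they stop, ending the chase.
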(event OnSeePawn(PawnSensing)
  (params (Pawn :type Pawn%20Object%20Reference))
  (bind _self self)
  (bind _returnvalue (AI|GetAIController _self))
  (bind _returnvalue_2 (AI|GetBlackboard _returnvalue))
  (Utilities|Casting|CastToBP_FirstPersonCharacter Pawn)
  (AI|Components|Blackboard|SetValueasBool _returnvalue_2 (Utilities|Name|MakeLiteralName "hasSeenPlayer") true)
  ;[1 1 1 1 10] set bool to false. if player is not seen, enemy wont chase player anymore. if player is still seen, enemy will continue chasing player
  (Utilities|FlowControl|RetriggerableDelay 0.6)
  (AI|Components|Blackboard|SetValueasBool _returnvalue_2 (Utilities|Name|MakeLiteralName "hasSeenPlayer") false))

(event EventBeginPlay
  (|CallParentFunction) ; This node is disabled and will not be called.\nDrag off pins to build functionality.
)

(event Collision|EventActorBeginOverlap
  (params (OtherActor :type Actor%20Object%20Reference))
  (|CallParentFunction OtherActor) ; This node is disabled and will not be called.\nDrag off pins to build functionality.
)

(event EventTick
  (params (DeltaSeconds :type Float%20%28single-precision%29))
  (|CallParentFunction DeltaSeconds) ; This node is disabled and will not be called.\nDrag off pins to build functionality.
)

(fn ConstructionScript
  (|CallParentFunction))