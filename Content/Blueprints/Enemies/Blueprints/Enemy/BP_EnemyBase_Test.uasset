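; Test-named elemental enemy AI character that patrols, chases, searches for and attacks the player with melee or ranged attacks.
; PawnSensing with a retriggerable delay sets Blackboard sight keys, and Tick runs attack range checks and a timed lost-player search.
; Attack events enable melee collision or fire element-specific bullets.
; BeginPlay picks a patrol area and its farthest point (despite MinDistance naming), while neighbour-average steering and capsule collision ignoring ease crowding.
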(event OnComponentBeginOverlap(AttackCollision)
  (params (OverlappedComponent :type Primitive%20Component%20Object%20Reference) (OtherActor :type Actor%20Object%20Reference) (OtherComp :type Primitive%20Component%20Object%20Reference) (OtherBodyIndex :type Integer) (bFromSweep :type Boolean) (SweepResult :type Hit%20Result%20Structure%20%28by%20ref%29))
  ;[1 1 1] Melee Collision
  ;;[1 1 1] check if collided into object is player
  (bind _asbp_first_person_character (Utilities|Casting|CastToBP_FirstPersonCharacter OtherActor))
  (bind _returnvalue (Game|Damage|ApplyDamage _asbp_first_person_character (Variables|Default|GetEnemyDamage) 0 0 "/Script/Engine.DamageType"))
  (if (> _returnvalue 0.0)
    (bind _returnvalue_2 (UserInterface|CreateWidget "/Game/UI/Player/HUD/Widgets/WBP_HitCircle.WBP_HitCircle_C" 0 _asbp_first_person_character (Transformation|GetActorLocation)))
    (UserInterface|Viewport|AddtoViewport _returnvalue_2 0)))

(event OnSeePawn(PawnSensing)
  (params (Pawn :type Pawn%20Object%20Reference))
  (bind _self self)
  (bind _returnvalue (AI|GetAIController _self))
  (bind _returnvalue_2 (AI|GetBlackboard _returnvalue))
  ;[1 1 1] sensing
  (Utilities|Casting|CastToBP_FirstPersonCharacter Pawn)
  (Variables|Default|SetCan%20Attack true)
  (Variables|Default|SetIs%20Chaseimg true)
  (AI|Components|Blackboard|SetValueasBool _returnvalue_2 (Utilities|Name|MakeLiteralName "hasSeenPlayer") true)
  ;;[1 1 1 1 10] set bool to false. if player is not seen, enemy wont chase player anymore. if player is still seen, enemy will continue chasing player
  (Utilities|FlowControl|RetriggerableDelay 0.6)
  ;;[1 1 1] Lost
  (Variables|Default|SetCan%20Attack false)
  (AI|Components|Blackboard|SetValueasBool _returnvalue_2 (Utilities|Name|MakeLiteralName "hasSeenPlayer") false))

(event OnComponentHit(CapsuleComponent)
  (params (HitComponent :type Primitive%20Component%20Object%20Reference) (OtherActor :type Actor%20Object%20Reference) (OtherComp :type Primitive%20Component%20Object%20Reference) (NormalImpulse :type Vector :default "0, 0, 0") (Hit :type Hit%20Result%20Structure%20%28by%20ref%29))
  ;[1 1 1] prevent enemy traffic jams
  (Utilities|Casting|CastToBP_EnemyBase OtherActor)
  (if (not (ScalableFloat|GetValueasBool (AI|GetBlackboard (AI|GetAIController self)) (Utilities|Name|MakeLiteralName "hasSeenPlayer")))
    (Collision|SetCollisionResponsetoChannel (Variables|Default|GetCapsuleComponent) "ECC_Pawn" "ECR_Ignore")))

(event OnHearNoise(PawnSensing)
  (params (Instigator :type Pawn%20Object%20Reference) (Location :type Vector%20%28by%20ref%29 :default "0, 0, 0") (Volume :type Float%20%28single-precision%29)))

(event Custom|Attack%20Melee
  ;[1 1 1] Melee
  (switch Utilities|FlowControl|Switch|SwitchonElement (Variables|Default|GetElement)
    (:NewEnumerator0
      (Audio|PlaySoundatLocation "/Game/Sound/SW_FireMeleeAttack.SW_FireMeleeAttack" "0, 0, 0" "0, 0, 0" 1.0 1.0 0.0 0 0 0 0))
    (:NewEnumerator1
      (Audio|PlaySoundatLocation "/Game/Sound/SW_WaterMeleeAttack.SW_WaterMeleeAttack" "0, 0, 0" "0, 0, 0" 1.0 1.0 0.0 0 0 0 0))
    (:NewEnumerator2
      (Audio|PlaySoundatLocation "/Game/Sound/SW_ElectricMeleeAttack.SW_ElectricMeleeAttack" "0, 0, 0" "0, 0, 0" 1.0 1.0 0.0 0 0 0 0)))
  (Collision|SetCollisionEnabled (Variables|Default|GetAttack%20Collision) "QueryAndPhysics"))

(event Custom|Lost%20Player%20Update
  (params (Delta%20Seconds :type Float%20%28double-precision%29))
  ;[1 1 1] Lost sight of player
  (if (not (ScalableFloat|GetValueasBool (AI|GetBlackboard (AI|GetAIController self)) (Utilities|Name|MakeLiteralName "hasSeenPlayer")))
    (if (Variables|Default|GetIs%20Chaseimg)
      (CallFunction|LostPlayer)
      (Variables|Default|SetIs%20Chaseimg false)
      (else
        ;;[1 1 1] Time to Search
        (if (ScalableFloat|GetValueasBool (AI|GetBlackboard (AI|GetAIController self)) (Utilities|Name|MakeLiteralName "lostPlayer"))
          (bind _output_get (Variables|Default|SetSearch%20Time (- (stale _output_get) Delta%20Seconds)))
          ;;[1 1 1] time over to search
          (if (> _output_get 0.0)
            (if (> _output_get 2.0)
              ;;[1 1 1] Lost Location Update
              (Variables|Default|SetLost%20Player%20Location (Transformation|GetActorLocation (Game|GetPlayerCharacter 0))))
            (else
              (AI|Components|Blackboard|SetValueasBool (AI|GetBlackboard (AI|GetAIController self)) (Utilities|Name|MakeLiteralName "lostPlayer") false)
              (Development|PrintString "patrol"))))))))

(event Custom|Lost%20Player
  ;[1 1 1] Lost sight of player
  ;;[1 1 1] Searching time
  (Variables|Default|SetSearch%20Time 3.0)
  (AI|Components|Blackboard|SetValueasBool (AI|GetBlackboard (AI|GetAIController self)) (Utilities|Name|MakeLiteralName "lostPlayer") true)
  (Development|PrintString "lost player")
  ;;[1 1 1] Lost Location Update
  (Variables|Default|SetLost%20Player%20Location (Transformation|GetActorLocation (Game|GetPlayerCharacter 0))))

(event Custom|Attack%20Ranged
  ;[1 1 1] Ranged
  (switch Utilities|FlowControl|Switch|SwitchonElement (Variables|Default|GetElement)
    (:NewEnumerator0
      (Audio|PlaySoundatLocation "/Game/Sound/SW_FireRangedAttack.SW_FireRangedAttack" "0, 0, 0" "0, 0, 0" 1.0 1.0 0.0 0 0 0 0))
    (:NewEnumerator1
      (Audio|PlaySoundatLocation "/Game/Sound/SW_WaterRangedAttack.SW_WaterRangedAttack" "0, 0, 0" "0, 0, 0" 1.0 1.0 0.0 0 0 0 0))
    (:NewEnumerator2
      (Audio|PlaySoundatLocation "/Game/Sound/SW_ElectricRangedAttack.SW_ElectricRangedAttack" "0, 0, 0" "0, 0, 0" 1.0 1.0 0.0 0 0 0 0)))
  (bind _returnvalue (Game|SpawnActorfromClass "/Game/Blueprints/Enemies/Blueprints/Enemy/BP_BulletBase.BP_BulletBase_C" (Math|Transform|MakeTransform (Transformation|GetSocketLocation (Variables|Character|GetMesh) "ShotTransform") (Math|Rotator|FindLookatRotation (Transformation|GetActorLocation) (Transformation|GetActorLocation (Game|Player|GetPlayerPawn 0))) "1.000000,1.000000,1.000000") "AlwaysSpawn" 0 0))
  (bind _output_get (Variables|Default|SetBullet _returnvalue))
  (Utilities|IsValid _output_get
    (:Is%20Valid
      (switch Utilities|FlowControl|Switch|SwitchonElement (Variables|Default|GetElement)
        (:NewEnumerator0
          (Development|SetHiddeninGame (Variables|/Game/Blueprints/Enemies/Blueprints/Enemy/BP_BulletBase.BP_BulletBase_C|GetFireFX (Variables|Default|GetBullet)) false false)
          (Effects|Components|ParticleSystem|SetFloatParameter (Variables|/Game/Blueprints/Enemies/Blueprints/Enemy/BP_BulletBase.BP_BulletBase_C|GetFireFX (Variables|Default|GetBullet)) "Velocity" 0.5)
          (Effects|Components|ParticleSystem|SetVectorParameter (Variables|/Game/Blueprints/Enemies/Blueprints/Enemy/BP_BulletBase.BP_BulletBase_C|GetFireFX (Variables|Default|GetBullet)) "Direction" "1.000000,0.000000,0.000000"))
        (:NewEnumerator1
          (Development|SetHiddeninGame (Variables|/Game/Blueprints/Enemies/Blueprints/Enemy/BP_BulletBase.BP_BulletBase_C|GetWaterFX (Variables|Default|GetBullet)) false false)
          (Effects|Components|ParticleSystem|SetFloatParameter (Variables|/Game/Blueprints/Enemies/Blueprints/Enemy/BP_BulletBase.BP_BulletBase_C|GetWaterFX (Variables|Default|GetBullet)) "Velocity" 0.5)
          (Effects|Components|ParticleSystem|SetVectorParameter (Variables|/Game/Blueprints/Enemies/Blueprints/Enemy/BP_BulletBase.BP_BulletBase_C|GetWaterFX (Variables|Default|GetBullet)) "Direction" "1.000000,0.000000,0.000000"))
        (:NewEnumerator2
          (Development|SetHiddeninGame (Variables|/Game/Blueprints/Enemies/Blueprints/Enemy/BP_BulletBase.BP_BulletBase_C|GetElectricFX (Variables|Default|GetBullet)) false false)
          (Effects|Components|ParticleSystem|SetFloatParameter (Variables|/Game/Blueprints/Enemies/Blueprints/Enemy/BP_BulletBase.BP_BulletBase_C|GetElectricFX (Variables|Default|GetBullet)) "Velocity" 0.5)
          (Effects|Components|ParticleSystem|SetVectorParameter (Variables|/Game/Blueprints/Enemies/Blueprints/Enemy/BP_BulletBase.BP_BulletBase_C|GetElectricFX (Variables|Default|GetBullet)) "Direction" "1.000000,0.000000,0.000000"))))))

(event Custom|Attack%20Cancel
  ;[1 1 1] Attack Collision Invalid
  (Variables|Default|SetIs%20Attacking false)
  (Collision|SetCollisionEnabled (Variables|Default|GetAttack%20Collision) "NoCollision"))

(event Custom|Attack%20Ranged%20End
  ;[1 1 1] Ranged
  (Variables|Default|SetIs%20Attacking false))

(event EventBeginPlay
  (|CallParentFunction)
  (CallFunction|SelectMyPatrolArea))

(event EventTick
  (params (DeltaSeconds :type Float%20%28single-precision%29))
  ;[1 1 1] check alive
  (if (> (Variables|Default|GetEnemyHealth) 0.0)
    (CallFunction|AttackCheck)
    (CallFunction|LostPlayerUpdate DeltaSeconds)
    (AI|Components|Blackboard|SetValueasBool (AI|GetBlackboard (AI|GetAIController self)) (Utilities|Name|MakeLiteralName "IsAttacking") (Variables|Default|GetIs%20Attacking))
    (CallFunction|SpreadCrowd)
    (CallFunction|UpdateState)))

(fn ConstructionScript
  (|CallParentFunction))

(fn AttackCheck
  (Components|Activation|SetActive (Variables|Character|GetCharacterMovement) true false)
  (if (Math|Boolean|ANDBoolean (Variables|Default|GetCan%20Attack) (not (Variables|Default|GetIs%20Attacking)) (ScalableFloat|GetValueasBool (AI|GetBlackboard (AI|GetAIController self)) (Utilities|Name|MakeLiteralName "hasSeenPlayer")) (Variables|Default|GetIs%20Chaseimg))
    ;[1 1 1] Check Enemy and Player DIstance
    (if (Variables|Default|GetAttack%20Type%20Melee)
      (if (<= (Math|Vector|Distance(Vector) (Transformation|GetActorLocation) (Transformation|GetActorLocation (Game|GetPlayerCharacter 0))) (Variables|Default|GetMelee%20Distance))
        (Variables|Default|SetIs%20Attacking true))
      (elif (<= (Math|Vector|Distance(Vector) (Transformation|GetActorLocation) (Transformation|GetActorLocation (Game|GetPlayerCharacter 0))) (Variables|Default|GetRanged%20Distance))
        (if (<= (Variables|Default|GetShot%20Cooldown) 0.0)
          (Variables|Default|SetIs%20Attacking true)
          ;[1 1 1] Add Cool Time
          (Variables|Default|SetShot%20Cooldown 2.0)
          (else
            ;[1 1 1] Count Cool Time
            (bind _output_get (Variables|Default|SetShot%20Cooldown (Math|Float|Clamp(Float) (- (stale _output_get) (Utilities|Time|GetWorldDeltaSeconds)) 0.0 2.0) :!label _label))))
        (else
          (goto _label))))
    (else
      ;[1 1 1] Attacking
      (if (Variables|Default|GetIs%20Attacking)
        (Transformation|SetActorRotation (Math|Rotator|MakeRotator 0.0 0.0 (.yaw (Math|Conversions|RotationFromXVector (- (Transformation|GetActorLocation (Game|GetPlayerCharacter 0)) (Transformation|GetActorLocation))))))
        (Components|Activation|SetActive (Variables|Character|GetCharacterMovement) false false)))))

(fn SelectMyPatrolArea
  ;[1 1 1] search area
  (bind _outactors (Actor|GetAllActorsOfClass "/Game/Blueprints/Enemies/Blueprints/Enemy/Patrol/BP_Patrol_Area.BP_Patrol_Area_C"))
  (bind _array_element (Utilities|Array|ForEachLoopwithBreak _outactors :!label _label)
    (:LoopBody
      (if (Default|CheckinRange (.AsBP%20Patrol%20Area (Utilities|Casting|CastToBP_Patrol_Area _array_element)) (Transformation|GetActorLocation))
        (Variables|Default|SetMy%20Patrol%20Area (.AsBP%20Patrol%20Area (Utilities|Casting|CastToBP_Patrol_Area _array_element)))
        (goto _label Break)))
    (:Completed
      (CallFunction|SelectFirstPatrolPoint)
      ;[1 1 1] Patrol or Random and Idol
      (AI|Components|Blackboard|SetValueasBool (AI|GetBlackboard (AI|GetAIController self)) (Utilities|Name|MakeLiteralName "IsHavingPatrolArea") (Utilities|IsValid (Variables|Default|GetMy%20Patrol%20Area))))))

(fn SelectFirstPatrolPoint
  (bind _my_patrol_area (Variables|Default|GetMy%20Patrol%20Area))
  ;[1 1 1] checking had patrol area data
  (if (Utilities|IsValid _my_patrol_area)
    (for (_array_element _array_index) (Variables|/Game/Blueprints/Enemies/Blueprints/Enemy/Patrol/BP_Patrol_Area.BP_Patrol_Area_C|GetPatrol%20Point%20List _my_patrol_area)
      (if (== _array_index 0)
        ;[1 1 1] first
        (LocalVariables|SetMin%20DIstance (Math|Vector|VectorLength (- (Transformation|GetActorLocation) (Transformation|GetActorLocation _array_element))))
        (Variables|Default|SetLast%20Passed%20Point%20Number 0)
        (elif (< (LocalVariables|GetMin%20DIstance) (Math|Vector|VectorLength (- (Transformation|GetActorLocation) (Transformation|GetActorLocation _array_element))))
          ;[1 1 1] Update
          (LocalVariables|SetMin%20DIstance (Math|Vector|VectorLength (- (Transformation|GetActorLocation) (Transformation|GetActorLocation _array_element))))
          (Variables|Default|SetLast%20Passed%20Point%20Number _array_index))))))

(fn SpreadCrowd
  (bind _outactors (Actor|GetAllActorsOfClass "/Game/Blueprints/Enemies/Blueprints/Enemy/BP_EnemyBase.BP_EnemyBase_C"))
  (for _array_element _outactors
    ;[1 1 1] searh near enemies
    (if (Variables|Default|GetIs%20Chaseimg)
      (if (<= (Math|Vector|VectorLength (- (Transformation|GetActorLocation _array_element) (Transformation|GetActorLocation))) 5e+01)
        (bind _output_get (LocalVariables|SetDifference%20Location (+ (stale _output_get) (Transformation|GetActorLocation _array_element)) :!label _label))
        (Math|Integer|IncrementInt (LocalVariables|GetCrowd%20Number)))
      (elif (<= (Math|Vector|VectorLength (- (Transformation|GetActorLocation _array_element) (Transformation|GetActorLocation))) 1e+02)
        (if (not (<= (Math|Vector|VectorLength (- (Transformation|GetActorLocation _array_element) (Transformation|GetActorLocation))) 5e+01))
          (goto _label)))))
  ;[1 1 1] Not only self
  (if (<= (LocalVariables|GetCrowd%20Number) 1)
    (bind _output_get_2 (Variables|Default|SetAvoiding%20Speed (* (stale _output_get_2) 0.5) :!label _label_2))
    (elif (== (Math|Vector|VectorLength (/ (LocalVariables|GetDifference%20Location) (LocalVariables|GetCrowd%20Number))) 0.0)
      (goto _label_2)
      (else
        (Variables|Default|SetAvoiding%20Speed 1.0)
        (bind _output_get_3 (Variables|Default|SetAvoiding%20Vector (- (Transformation|GetActorLocation) (/ (LocalVariables|GetDifference%20Location) (LocalVariables|GetCrowd%20Number))))))))
  (Pawn|Input|AddMovementInput _output_get_3 (Variables|Default|GetAvoiding%20Speed) false))

(fn ChangeElement
  (bind _enemy_head_ref (Variables|Default|GetEnemy%20Head%20REF))
  ;[1 1 1] Change element
  (Utilities|FlowControl|Sequence
    (:then_0
      (switch int (Math|Random|RandomIntegerinRange 0 2)
        (:0
          (bind _output_get (Variables|Default|SetElement "NewEnumerator0"))
          (Variables|/Game/Blueprints/Enemies/Blueprints/EnemyHead/BP_EnemyHeadBase.BP_EnemyHeadBase_C|SetElement _enemy_head_ref _output_get))
        (:1
          (bind _output_get_2 (Variables|Default|SetElement "NewEnumerator1"))
          (Variables|/Game/Blueprints/Enemies/Blueprints/EnemyHead/BP_EnemyHeadBase.BP_EnemyHeadBase_C|SetElement _enemy_head_ref _output_get_2))
        (:2
          (bind _output_get_3 (Variables|Default|SetElement "NewEnumerator2"))
          (Variables|/Game/Blueprints/Enemies/Blueprints/EnemyHead/BP_EnemyHeadBase.BP_EnemyHeadBase_C|SetElement _enemy_head_ref _output_get_3))))
    (:then_1
      (Default|ChangeColour _enemy_head_ref))))

(fn UpdateState
  (if (not (Variables|Default|GetIs%20Chaseimg))
    (if (ScalableFloat|GetValueasBool (AI|GetBlackboard (AI|GetAIController self)) (Utilities|Name|MakeLiteralName "lostPlayer"))
      _)))