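; BP_BoidManager spawns and drives a flock of BP_Boid actors.
; On BeginPlay it spawns SpawnAmount boids at random points inside its Box component and stores them in an array.
; Each Tick it calls Flock on every boid with shared alignment, cohesion and separation weights and radii, then MoveBoid, so the manager centrally updates the classic boids simulation.
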(event EventBeginPlay
  (bind _box (Variables|Default|GetBox))
  (for _index (range 1 (Variables|Default|GetSpawnAmount))
    (bind _returnvalue (Game|SpawnActorfromClass "/Game/Blueprints/Enemies/Blueprints/Others/BP_Boid.BP_Boid_C" (Math|Transform|MakeTransform (Math|Random|RandomPointinBoundingBox (Transformation|GetWorldLocation _box) (Variables|/Script/Engine.BoxComponent|GetBoxExtent _box)) "0, 0, 0" "1.000000,1.000000,1.000000") "AdjustIfPossibleButAlwaysSpawn" 0 0))
    (Utilities|Array|Add (Variables|Default|GetArray) _returnvalue)))

(event EventTick
  (params (DeltaSeconds :type Float%20%28single-precision%29))
  (for _array_element (Variables|Default|GetArray)
    (Default|Flock _array_element (Variables|Default|GetAlignment%20Multiplier) (Variables|Default|GetCohesion%20Mulitplier) (Variables|Default|GetSeparation%20Multiplier) (Variables|Default|GetAlignment%20Radius) (Variables|Default|GetCohesion%20Radius) (Variables|Default|GetSeparation%20Radius))
    (Default|MoveBoid _array_element)))

(fn ConstructionScript)