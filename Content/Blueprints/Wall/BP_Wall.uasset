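; BP_Wall is a wall actor that caches its Cube's world location at BeginPlay to act as a repulsion point for boids.
; Separate sums distance-weighted steering from that point to every boid within PerceptionRadius, flattening the running Z before each addition.
; After the loop, it averages that sum, converts it to a clamped steering force and adds it only to the last array element's acceleration.
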(event EventBeginPlay
  (Variables|Default|Setposition (Transformation|GetWorldLocation (Variables|Default|GetCube))))

(event Collision|EventActorBeginOverlap
  (params (OtherActor :type Actor%20Object%20Reference)))

(event EventTick
  (params (DeltaSeconds :type Float%20%28single-precision%29)))

(fn ConstructionScript)

(fn Separate
  (params (BoidArray :type Array%20of%20BP%20Boid%20Object%20References))
  (for _array_element BoidArray
    (bind _output_get (LocalVariables|Setdistance (Math|Vector|Distance(Vector) (Variables|Default|Getposition) (Variables|/Game/Blueprints/Enemies/Blueprints/Others/BP_Boid.BP_Boid_C|Getposition _array_element))))
    (if (< (LocalVariables|Getdistance) (LocalVariables|GetperceptionRadius))
      (bind _output_get_2 (LocalVariables|Setdiff (- (Variables|Default|Getposition) (Variables|/Game/Blueprints/Enemies/Blueprints/Others/BP_Boid.BP_Boid_C|Getposition _array_element))))
      (LocalVariables|Setsteering (+ (Math|Vector|MakeVector (.x (LocalVariables|Getsteering)) (.y (LocalVariables|Getsteering)) 0.0) (/ _output_get_2 _output_get)))
      (Math|Integer|IncrementInt (LocalVariables|Gettotal))))
  (if (> (LocalVariables|Gettotal) 0)
    (bind _output_get_3 (LocalVariables|Setsteering (/ (LocalVariables|Getsteering) (LocalVariables|Gettotal))))
    (bind _output_get_4 (LocalVariables|Setsteering (- (* (Math|Vector|Normalize _output_get_3) (.x (Variables|Default|GetmaxSpeed))) (Variables|/Game/Blueprints/Enemies/Blueprints/Others/BP_Boid.BP_Boid_C|Getvelocity _array_element))))
    (bind _output_get_5 (LocalVariables|Setseparation (Math|Vector|VectorClampSizeMax _output_get_4 (.x (Variables|Default|GetmaxForce)))))
    (Variables|/Game/Blueprints/Enemies/Blueprints/Others/BP_Boid.BP_Boid_C|Setacceleration _array_element (+ (Variables|/Game/Blueprints/Enemies/Blueprints/Others/BP_Boid.BP_Boid_C|Getacceleration _array_element) _output_get_5))))