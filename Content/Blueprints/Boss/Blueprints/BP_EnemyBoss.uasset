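; Boss enemy character with projectile, projectile rain, swept laser, hand swipe and hand slam attacks, run by a behavior tree once activated.
; Attacks are callable events and functions using socket spawns, shuffled spawn points, an overlap box, sphere overlaps and a per-tick sphere trace.
; Low health triggers a one-time shield and widget, setting a blackboard Heal flag until healing stops.
; Lethal damage shows the win screen and pauses the game.
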(event OnComponentBeginOverlap(HandSwipeBox)
  (params (OverlappedComponent :type Primitive%20Component%20Object%20Reference) (OtherActor :type Actor%20Object%20Reference) (OtherComp :type Primitive%20Component%20Object%20Reference) (OtherBodyIndex :type Integer) (bFromSweep :type Boolean) (SweepResult :type Hit%20Result%20Structure%20%28by%20ref%29))
  (bind _handswipebox (Variables|Default|GetHandSwipeBox))
  (bind _returnvalue (Transformation|GetWorldLocation _handswipebox))
  ;[1 1 1 1 30] check when boss does hand swipe attack, if box collider hits player
  (if (Variables|Default|GetisHandSwiping)
    (bind _asbp_first_person_character (Utilities|Casting|CastToBP_FirstPersonCharacter OtherActor))
    (Game|Damage|ApplyDamage _asbp_first_person_character 5e+01 0 0)
    (Utilities|FlowControl|DoOnce false
      (:Completed
        ;;[1 1 1] add knockback to player if hit
        (Character|LaunchCharacter _asbp_first_person_character (Math|Vector|MakeVector (* (.x (- (Transformation|GetWorldLocation (Variables|/Script/Engine.Actor|GetRootComponent _asbp_first_person_character)) _returnvalue)) 15.0) (* (Math|Float|MakeLiteralFloat 5e+01) 3e+01) (* (Math|Float|MakeLiteralFloat 2e+01) 1e+01)) false false)
        (Camera|PlayWorldCameraShake "/Game/FirstPerson/Blueprints/BP_HeavyCameraShake.BP_HeavyCameraShake_C" _returnvalue 0.0 1e+03)))))

(event Custom|ShowHitEffect
  (params (Location :type Vector))
  ;[1 1 1] Show hit effect for boss
  (bind _returnvalue (AddComponent|AddWidgetComponent true (Math|Transform|MakeTransform Location "0, 0, 0" "1.000000,1.000000,1.000000")))
  (Utilities|FlowControl|Delay 0.2)
  (Components|DestroyComponent _returnvalue))

(event Custom|HandSwipeEvent
  (params (Left :type Boolean))
  ;[1 1 1] Hand Swipe Start
  (Variables|Default|SetisHandSwiping true)
  (if Left
    (Transformation|AttachComponentToComponent (Variables|Default|GetHandSwipeBox) (Variables|Character|GetMesh) "LeftHandSwipeTransform" "SnapToTarget" "SnapToTarget" "SnapToTarget" true)
    (else
      (Transformation|AttachComponentToComponent (Variables|Default|GetHandSwipeBox) (Variables|Character|GetMesh) "RightHandSwipeTransform" "SnapToTarget" "SnapToTarget" "SnapToTarget" true))))

(event Custom|RainProjectilesAttack
  (bind _spawnpointarray (Variables|Default|GetSpawnPointArray))
  ;[1 1 1] Rain Projectiles Attack
  ;;[1 1 1] randomize locations to spawn projectiles
  (Utilities|Array|Shuffle _spawnpointarray)
  (bind _array_element (Utilities|Array|ForEachLoopwithBreak _spawnpointarray :!label _label)
    (:LoopBody
      (Game|SpawnActorfromClass "/Game/Blueprints/Boss/Blueprints/BP_ProjectileSpawnArea.BP_ProjectileSpawnArea_C" (Math|Transform|MakeTransform (Transformation|GetWorldLocation _array_element) "0, 0, 0" "5.000000,5.000000,0.050000") "AdjustIfPossibleButAlwaysSpawn" 0 0)
      (bind _result (Math|Integer|IncrementInt (Variables|Default|GetSpawnCounter))
        (:%20%20
          (bind _output_get (Variables|Default|SetSpawnCounter _result))
          (if (> _output_get 4)
            (goto _label Break)))))
    (:Completed
      (Variables|Default|SetSpawnCounter 0))))

(event Custom|HandSwipeEventEnd
  ;[1 1 1] Hand Swipe Start
  ;;[1 1 1] Hand Swipe Stop
  (Variables|Default|SetisHandSwiping false))

(event Custom|Create%20Projectiles
  ;[1 1 1] Projectile Attack
  (Game|SpawnActorfromClass "/Game/Blueprints/Boss/Blueprints/BP_BossProjectile.BP_BossProjectile_C" (Transformation|GetSocketTransform (Variables|Character|GetMesh) "SpawnTransform1" "RTS_World") "AdjustIfPossibleButAlwaysSpawn" 0 0)
  (Game|SpawnActorfromClass "/Game/Blueprints/Boss/Blueprints/BP_BossProjectile.BP_BossProjectile_C" (Transformation|GetSocketTransform (Variables|Character|GetMesh) "SpawnTransform2" "RTS_World") "AdjustIfPossibleButAlwaysSpawn" 0 0))

(event Custom|Heal
  (bind _output_get (Variables|Default|SetBoss%20Health (+ (Variables|Default|GetBoss%20Health) 2.0)))
  (if (> _output_get (Variables|Default|GetAmount%20to%20Heal%20To))
    (CallFunction|StopHealing)))

(event Custom|Stop%20Healing
  (AI|Components|Blackboard|SetValueasBool (AI|GetBlackboard (AI|GetAIController self)) (Utilities|Name|MakeLiteralName "Heal") false)
  (Actor|DestroyActor (Variables|Default|GetShield%20REF))
  (Widget|RemovefromParent (Variables|Default|GetShield%20Widget%20REF)))

(event EventBeginPlay
  ;[1 1 1] Add spawn points for rain projectiles attack to an array
  (Utilities|FlowControl|Sequence
    (:then_0
      (Variables|Default|SetSpawnPointArray (Utilities|Array|MakeArray (Variables|Default|GetSpawnPoint1) (Variables|Default|GetSpawnPoint2) (Variables|Default|GetSpawnPoint3) (Variables|Default|GetSpawnPoint4) (Variables|Default|GetSpawnPoint5) (Variables|Default|GetSpawnPoint6) (Variables|Default|GetSpawnPoint7) (Variables|Default|GetSpawnPoint8) (Variables|Default|GetSpawnPoint9) (Variables|Default|GetSpawnPoint10))))))

(event EventTick
  (params (DeltaSeconds :type Float%20%28single-precision%29))
  ;[1 1 1] Laser Attack
  (CallFunction|LaserAttack DeltaSeconds))

(event Game|Damage|EventAnyDamage
  (params (Damage :type Float%20%28single-precision%29) (DamageType :type Damage%20Type%20Object%20Reference) (InstigatedBy :type Controller%20Object%20Reference) (DamageCauser :type Actor%20Object%20Reference))
  (if (<= (- (Variables|Default|GetBoss%20Health) Damage) 0.0)
    (bind _returnvalue (UserInterface|CreateWidget "/Game/UI/WinLoseScreen/Widgets/WBP_WinScreen.WBP_WinScreen_C"))
    (UserInterface|Viewport|AddtoViewport _returnvalue 0)
    (Game|SetGamePaused true)
    (else
      (bind _output_get (Variables|Default|SetBoss%20Health (Math|Float|Clamp(Float) (- (Variables|Default|GetBoss%20Health) Damage) 0.0 (Variables|Default|GetBoss%20Max%20Health))))
      (if (<= _output_get 1.5e+02)
        (Utilities|FlowControl|DoOnce false
          (:Completed
            (Variables|Default|SetAmount%20to%20Heal%20To (+ (Variables|Default|GetBoss%20Health) 1e+02))
            (bind _returnvalue_2 (Game|SpawnActorfromClass "/Game/Blueprints/Boss/Blueprints/BP_EnemyBossShield.BP_EnemyBossShield_C" (Transformation|GetSocketTransform (Variables|Character|GetMesh) "ShieldTransform" "RTS_World") "Undefined" 0 0))
            (bind _output_get_2 (Variables|Default|SetShield%20REF _returnvalue_2))
            (if (<= _output_get 5e+01)
              (bind _output_get_3 (Variables|/Game/Blueprints/Boss/Blueprints/BP_EnemyBossShield.BP_EnemyBossShield_C|SetShield%20Health _output_get_2 5))
              (Variables|/Game/Blueprints/Boss/Blueprints/BP_EnemyBossShield.BP_EnemyBossShield_C|SetMax%20Shield%20Health _output_get_2 _output_get_3)
              (else
                (bind _output_get_4 (Variables|/Game/Blueprints/Boss/Blueprints/BP_EnemyBossShield.BP_EnemyBossShield_C|SetShield%20Health _output_get_2 3))
                (Variables|/Game/Blueprints/Boss/Blueprints/BP_EnemyBossShield.BP_EnemyBossShield_C|SetMax%20Shield%20Health _output_get_2 _output_get_4)))
            (Transformation|AttachComponentToComponent _output_get_2 (Variables|Character|GetMesh) "ShieldTransform" "SnapToTarget" "SnapToTarget" "SnapToTarget" true)
            (bind _output_get_5 (Variables|/Game/Blueprints/Boss/Blueprints/BP_EnemyBossShield.BP_EnemyBossShield_C|SetBoss%20REF _output_get_2 self))
            (bind _returnvalue_3 (UserInterface|CreateWidget "/Game/UI/Boss/Widgets/WBP_BossShield.WBP_BossShield_C" 0 _output_get_5))
            (bind _output_get_6 (Variables|Default|SetShield%20Widget%20REF _returnvalue_3))
            (UserInterface|Viewport|AddtoViewport _output_get_6 0)
            (AI|Components|Blackboard|SetValueasBool (AI|GetBlackboard (AI|GetAIController self)) (Utilities|Name|MakeLiteralName "Heal") true)))))))

(fn ConstructionScript)

(fn LaserAttack
  (params (Alpha :type Float%20%28single-precision%29))
  (bind _returnvalue (Math|Rotator|MakeRotator 0.0 -2e+01 9e+01))
  (bind _returnvalue_2 (* Alpha 5.0))
  (bind _laserpoint (Variables|Default|GetLaserPoint))
  (bind _laserpoint_2 (Variables|Default|GetLaserPoint))
  (bind _returnvalue_3 (Transformation|GetWorldLocation _laserpoint))
  (bind _relativerotation (Variables|/Script/Engine.SceneComponent|GetRelativeRotation _laserpoint_2))
  (bind _returnvalue_4 (Math|Rotator|Lerp(Rotator) _relativerotation _returnvalue _returnvalue_2))
  (if (Variables|Default|GetcanLaserAttack)
    ;[1 1 1] sphere trace from the position of the arrow
    (bind (_outhit _returnvalue_5) (Collision|SphereTraceForObjects _returnvalue_3 (+ _returnvalue_3 (* (Math|Vector|GetForwardVector (Transformation|GetWorldRotation _laserpoint)) 5e+03)) 2e+01 (Utilities|Array|MakeArray "ObjectTypeQuery3") false 0 "ForDuration" true "(R=1.000000,G=0.000000,B=0.000000,A=1.000000)" "(R=0.000000,G=1.000000,B=0.000000,A=1.000000)" 0.1))
    ;[1 1 1] lerp the arrow + sphere trace
    (Transformation|SetWorldRotation _laserpoint_2 _returnvalue_4 false false)
    ;[1 1 1] check whether hit player
    (if _returnvalue_5
      (bind _asbp_first_person_character (Utilities|Casting|CastToBP_FirstPersonCharacter (.HitActor (Collision|BreakHitResult _outhit))))
      (Game|Damage|ApplyDamage _asbp_first_person_character 7.0 0 0))
    (if (Utilities|Operators|EqualEqual _returnvalue_4 _returnvalue 0.5)
      (Variables|Default|SetcanLaserAttack false)
      (CallFunction|ResetLaserPosition)
      (return))))

(fn ResetLaserPosition
  (Transformation|SetWorldRotation (Variables|Default|GetLaserPoint) (Variables|Default|GetDefaultLaserPosition) false false))

(fn HandSlamAttack
  (params (SlamSide :type Boolean))
  (if SlamSide
    (Variables|Default|SetSlamAreaInfo (Variables|Default|GetLeftHandSlamArea))
    (else
      (Variables|Default|SetSlamAreaInfo (Variables|Default|GetRightHandSlamArea))))
  (Effects|SpawnEmitteratLocation "/Game/StarterContent/Particles/P_Explosion.P_Explosion" (Transformation|GetWorldLocation (Variables|Default|GetSlamAreaInfo)) "0, 0, 0" "5.000000,5.000000,5.000000")
  (bind (_outactors _returnvalue) (Collision|SphereOverlapActors (Transformation|GetWorldLocation (Variables|Default|GetSlamAreaInfo)) (Variables|/Script/Engine.SphereComponent|GetSphereRadius (Variables|Default|GetSlamAreaInfo)) (Utilities|Array|MakeArray "ObjectTypeQuery3") 0 (Utilities|Array|MakeArray self)))
  (if _returnvalue
    (bind _asbp_first_person_character (Utilities|Casting|CastToBP_FirstPersonCharacter (Utilities|Array|Get(acopy) _outactors)))
    (Physics|AddImpulse (Variables|/Script/Engine.Character|GetCharacterMovement _asbp_first_person_character) (* (- (Transformation|GetWorldLocation (Variables|/Script/Engine.Character|GetMesh _asbp_first_person_character)) (Transformation|GetWorldLocation (Variables|Default|GetSlamAreaInfo))) "4000.000000,4000.000000,5000.000000") false)
    (Game|Damage|ApplyDamage _asbp_first_person_character 2e+01 0 0)
    (Camera|PlayWorldCameraShake "/Game/FirstPerson/Blueprints/BP_HeavyCameraShake.BP_HeavyCameraShake_C" (Transformation|GetWorldLocation (Variables|Default|GetSlamAreaInfo)) 0.0 5e+02)
    (else
      (Camera|PlayWorldCameraShake "/Game/FirstPerson/Blueprints/BP_LightCameraShake.BP_LightCameraShake_C" (Transformation|GetWorldLocation (Variables|Default|GetSlamAreaInfo)) 0.0 2.5e+03))))

(fn ActivateBoss
  (Variables|Default|SetAIControllerClass "/Game/Blueprints/Boss/AI/BP_BossAI_Controller.BP_BossAI_Controller_C")
  (Pawn|SpawnDefaultController)
  (AI|RunBehaviorTree (AI|GetAIController self) "/Game/Blueprints/Boss/AI/BT_BossAI.BT_BossAI"))