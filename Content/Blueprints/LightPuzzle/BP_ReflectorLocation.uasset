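; Light puzzle socket that acts as a laser source or reflector once the player places its matching item with F.
; Each tick a sphere overlap finds the player, and Q/E pitch, yaw or slide it depending on item type.
; An active caster line-traces with growing range to drive Niagara beam and impact effects.
; Hit reflectors relay the beam through a flag cleared every tick; hitting a BP_LightTarget only prints.
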(event EventBeginPlay
  (Effects|Components|ParticleSystem|SetColorParameter (Variables|Default|GetNiagaraLaser) "Color" "(R=0.827089,G=0.005004,B=1.000000,A=1.000000)"))

(event Collision|EventActorBeginOverlap
  (params (OtherActor :type Actor%20Object%20Reference)))

(event EventTick
  (params (DeltaSeconds :type Float%20%28single-precision%29))
  (CallFunction|CheckPlayer)
  (CallFunction|CheckItemAttached DeltaSeconds)
  (CallFunction|ChangeColour)
  (Variables|Default|SetisHitbyLight false)
  (if (< (Variables|Default|GetLight%20Range) 5e+03)
    (Variables|Default|SetLight%20Range (+ (Variables|Default|GetLight%20Range) (* 0.0 2e+03)))))

(fn ConstructionScript)

(fn CheckPlayer
  (bind _returnvalue (Game|GetPlayerController 0))
  (bind _returnvalue_2 (Game|GetPlayerController 0))
  (bind _cube (Variables|Default|GetCube))
  (bind _defaultsceneroot (Variables|Default|GetDefaultSceneRoot))
  (bind _returnvalue_3 (Transformation|GetWorldLocation _cube))
  (bind _returnvalue_4 (Game|Player|IsInputKeyDown _returnvalue "F"))
  (bind _returnvalue_5 (Game|Player|IsInputKeyDown _returnvalue_2 "Q"))
  (bind _returnvalue_6 (Transformation|GetWorldLocation _defaultsceneroot))
  (bind _returnvalue_7 (Game|Player|IsInputKeyDown _returnvalue_2 "E"))
  (bind _returnvalue_8 (Math|Conversions|ToInteger(Boolean) _returnvalue_4))
  ;[1 1 1] Check if Player is in radius of object
  (Rendering|Debug|DrawDebugSphere _returnvalue_3 2e+02 12 "(R=1.000000,G=1.000000,B=1.000000,A=1.000000)" 0.0)
  (bind _outactors (Collision|SphereOverlapActors _returnvalue_3 2e+02 (Variables|Default|GetObject%20Types) 0))
  (for _array_element _outactors
    (bind _asbp_first_person_character (Utilities|Casting|CastToBP_FirstPersonCharacter _array_element))
    (Utilities|FlowControl|Sequence
      (:then_0
        (if (Math|Conversions|ToBoolean(Integer) (Class|KismetMathLibrary|AndIntInt (Class|KismetMathLibrary|AndIntInt (Math|Conversions|ToInteger(Boolean) (Variables|/Game/FirstPerson/Blueprints/BP_FirstPersonCharacter.BP_FirstPersonCharacter_C|GetIsHavingItem1 _asbp_first_person_character)) _returnvalue_8) (Math|Conversions|ToInteger(Boolean) (Utilities|Enum|Equal(Enum) (Variables|Default|GetItem) (Utilities|Enum|LiteralenumItems "NewEnumerator0")))))
          (Variables|/Game/FirstPerson/Blueprints/BP_FirstPersonCharacter.BP_FirstPersonCharacter_C|SetIsHavingItem1 _asbp_first_person_character false)
          (Rendering|SetVisibility (Variables|Default|GetLight%20Caster) true true)
          (Variables|Default|SetisItem1Attached? true)
          (elif (Math|Conversions|ToBoolean(Integer) (Class|KismetMathLibrary|AndIntInt (Class|KismetMathLibrary|AndIntInt (Math|Conversions|ToInteger(Boolean) (Variables|/Game/FirstPerson/Blueprints/BP_FirstPersonCharacter.BP_FirstPersonCharacter_C|GetIsHavingItem2 _asbp_first_person_character)) _returnvalue_8) (Math|Conversions|ToInteger(Boolean) (Utilities|Enum|Equal(Enum) (Variables|Default|GetItem) (Utilities|Enum|LiteralenumItems "NewEnumerator1")))))
            (Variables|/Game/FirstPerson/Blueprints/BP_FirstPersonCharacter.BP_FirstPersonCharacter_C|SetIsHavingItem2 _asbp_first_person_character false)
            (Rendering|SetVisibility (Variables|Default|GetLight%20Caster) true true)
            (Variables|Default|SetisItem2Attached? true)
            (elif (Math|Conversions|ToBoolean(Integer) (Class|KismetMathLibrary|AndIntInt (Class|KismetMathLibrary|AndIntInt (Math|Conversions|ToInteger(Boolean) (Variables|/Game/FirstPerson/Blueprints/BP_FirstPersonCharacter.BP_FirstPersonCharacter_C|GetIsHavingItem3 _asbp_first_person_character)) _returnvalue_8) (Math|Conversions|ToInteger(Boolean) (Utilities|Enum|Equal(Enum) (Variables|Default|GetItem) (Utilities|Enum|LiteralenumItems "NewEnumerator2")))))
              (Variables|/Game/FirstPerson/Blueprints/BP_FirstPersonCharacter.BP_FirstPersonCharacter_C|SetIsHavingItem3 _asbp_first_person_character false)
              (Rendering|SetVisibility (Variables|Default|GetLight%20Caster) true true)
              (Variables|Default|SetisItem3Attached? true)))))
      (:then_1
        (if (Variables|Default|GetisItem1Attached?)
          (if _returnvalue_5
            (bind _output_get (Variables|Default|SetlightCasterYRot (+ (stale _output_get) 0.1)))
            (Transformation|SetRelativeRotation (Variables|Default|GetLight%20Caster) (Math|Rotator|MakeRotator 0.0 (Variables|Default|GetlightCasterYRot) 0.0) false false :!label _label)
            (elif _returnvalue_7
              (bind _output_get_2 (Variables|Default|SetlightCasterYRot (- (stale _output_get_2) 0.1)))
              (goto _label)))
          (elif (Variables|Default|GetisItem2Attached?)
            (if _returnvalue_7
              (bind _output_get_3 (Variables|Default|SetlightCasterZRot (+ (stale _output_get_3) 0.1)))
              (Transformation|SetRelativeRotation (Variables|Default|GetLight%20Caster) (Math|Rotator|MakeRotator 0.0 0.0 (Variables|Default|GetlightCasterZRot)) false false :!label _label_2)
              (elif _returnvalue_5
                (bind _output_get_4 (Variables|Default|SetlightCasterZRot (- (stale _output_get_4) 0.1)))
                (goto _label_2)))
            (elif (Variables|Default|GetisItem3Attached?)
              (if _returnvalue_7
                (Variables|Default|SetitemLocationYPos (.y _returnvalue_6))
                (bind _output_get_5 (Variables|Default|SetitemLocationYPos (+ (stale _output_get_5) 1.0)))
                (Transformation|SetActorLocation (Math|Vector|MakeVector (.x _returnvalue_6) (Variables|Default|GetitemLocationYPos) (.z _returnvalue_6)) true false :!label _label_3)
                (elif _returnvalue_5
                  (Variables|Default|SetitemLocationYPos (.y _returnvalue_6))
                  (bind _output_get_6 (Variables|Default|SetitemLocationYPos (- (stale _output_get_6) 1.0)))
                  (goto _label_3))))))))))

(fn CastLight
  (params (dt :type Float%20%28double-precision%29))
  (bind _light_caster (Variables|Default|GetLight%20Caster))
  (bind _niagaralaserimpact (Variables|Default|GetNiagaraLaserImpact))
  (bind _returnvalue (Transformation|GetWorldLocation _light_caster))
  (Utilities|FlowControl|Sequence
    (:then_0
      (bind _outhit (Collision|LineTraceForObjects _returnvalue (+ _returnvalue (* (Math|Vector|GetForwardVector (Transformation|GetWorldRotation _light_caster)) (Variables|Default|GetLight%20Range))) (Variables|Default|GetObject%20Types) false 0 "None" true "(R=0.028752,G=0.000000,B=1.000000,A=1.000000)" "(R=1.000000,G=0.000000,B=0.057065,A=1.000000)" 0.1))
      (Effects|Components|ParticleSystem|SetVectorParameter (Variables|Default|GetNiagaraLaser) "LaserEnd" (select (.bBlockingHit (Collision|BreakHitResult _outhit)) (.Location (Collision|BreakHitResult _outhit)) (+ _returnvalue (* (Math|Vector|GetForwardVector (Transformation|GetWorldRotation _light_caster)) (Variables|Default|GetLight%20Range)))))
      (Rendering|SetVisibility _niagaralaserimpact (.bBlockingHit (Collision|BreakHitResult _outhit)) false)
      (Transformation|SetWorldLocation _niagaralaserimpact (.Location (Collision|BreakHitResult _outhit)) false false)
      (Utilities|Casting|CastToBP_LightTarget (.HitActor (Collision|BreakHitResult _outhit))
        (:then
          (Development|PrintString "HIT"))
        (:CastFailed
          (bind _output_get (Variables|Default|SetLightSourceHitActorREF (.HitActor (Collision|BreakHitResult _outhit))))
          (bind _asbp_reflector_location (Utilities|Casting|CastToBP_ReflectorLocation _output_get))
          (Variables|BP_ReflectorLocation_C|SetisHitbyLight _asbp_reflector_location true)
          (Variables|BP_ReflectorLocation_C|SetisCastingRay? _asbp_reflector_location true))))
    (:then_1
      (if (< (Variables|Default|GetLight%20Range) 3e+03)
        (bind _output_get_2 (Variables|Default|SetLight%20Range (+ (stale _output_get_2) (* dt 1e+03))))))))

(fn CheckItemAttached
  (params (dt :type Float%20%28double-precision%29))
  (bind _islightsource (Variables|Default|GetisLightSource))
  (if _islightsource
    (if (Math|Conversions|ToBoolean(Integer) (Class|KismetMathLibrary|OrIntInt (Math|Conversions|ToInteger(Boolean) (Variables|Default|GetisItem1Attached?)) (Math|Conversions|ToInteger(Boolean) (Variables|Default|GetisItem2Attached?)) (Math|Conversions|ToInteger(Boolean) (Variables|Default|GetisItem3Attached?))))
      (CallFunction|CastLight dt)
      (Rendering|SetVisibility (Variables|Default|GetNiagaraLaser) _islightsource false))
    (elif (Math|Conversions|ToBoolean(Integer) (Class|KismetMathLibrary|AndIntInt (Math|Conversions|ToInteger(Boolean) (Math|Conversions|ToBoolean(Integer) (Class|KismetMathLibrary|AndIntInt (Math|Conversions|ToInteger(Boolean) (Variables|Default|GetisHitbyLight)) (Math|Conversions|ToInteger(Boolean) (Variables|Default|GetisCastingRay?))))) (Math|Conversions|ToInteger(Boolean) (Variables|/Script/Engine.SceneComponent|GetbVisible (Variables|Default|GetLight%20Caster)))))
      (CallFunction|CastLight dt)
      (Rendering|SetVisibility (Variables|Default|GetNiagaraLaser) true false)
      (elif (== (Variables|Default|GetisCastingRay?) false)
        (Rendering|SetVisibility (Variables|Default|GetNiagaraLaser) false false)
        (Rendering|SetVisibility (Variables|Default|GetNiagaraLaserImpact) false false)
        (Variables|Default|SetLight%20Range 0.0)))))

(fn ChangeColour
  (if (Variables|Default|GetisHitbyLight)
    (Rendering|Material|SetMaterial (Variables|Default|GetLight%20Caster) 0 "/Game/Blueprints/Enemies/MaterialsForHead/ElectricMaterial.ElectricMaterial" :!label _label)
    (elif (Variables|Default|GetisLightSource)
      (goto _label)
      (else
        (Rendering|Material|SetMaterial (Variables|Default|GetLight%20Caster) 0 "/Game/Assets/FPWeapon/Materials/BaseMaterial.BaseMaterial")
        (Variables|Default|SetLight%20Range 0.0)
        (Rendering|SetVisibility (Variables|Default|GetNiagaraLaser) false false)))))