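; BP_Door is a door actor that dissolves away and removes itself from the level.
; Its DissolveDoor event plays a timeline that drives the Power and Dissolve scalar parameters on the Door component's materials each update.
; When the timeline finishes, DestroyDoor destroys the actor.
; Nothing in this Blueprint triggers the dissolve, as overlap, tick and construction logic are empty.
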(event Custom|DestroyDoor
  (Actor|DestroyActor))

(event Custom|DissolveDoor
  (bind (_direction _dissolve_emission _power) (Timeline|Dissolve%20Door Play)
    (:Update
      (Rendering|Material|SetScalarParameterValueonMaterials (Variables|Default|GetDoor) "Power" _power)
      (Rendering|Material|SetScalarParameterValueonMaterials (Variables|Default|GetDoor) "Dissolve" _dissolve_emission))
    (:Finished
      (CallFunction|DestroyDoor))))

(event EventBeginPlay)

(event Collision|EventActorBeginOverlap
  (params (OtherActor :type Actor%20Object%20Reference)))

(event EventTick
  (params (DeltaSeconds :type Float%20%28single-precision%29)))

(fn ConstructionScript)