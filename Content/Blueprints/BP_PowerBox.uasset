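; Power box actor that displays which generators are activated on six indicator lights.
; Every Tick it polls GeneratorArray and swaps the light matching each active generator's OrderIndex to a shared material.
; Lights are never reverted by the poll; ResetLight, not called within this Blueprint, restores each light's own material and calls ResetEmissionValue on every generator.
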(event EventBeginPlay)

(event Collision|EventActorBeginOverlap
  (params (OtherActor :type Actor%20Object%20Reference)))

(event EventTick
  (params (DeltaSeconds :type Float%20%28single-precision%29))
  (CallFunction|ChangePowerBoxLight (Variables|Default|GetGeneratorArray)))

(fn ConstructionScript)

(fn ChangePowerBoxLight
  (params (GeneratorArray :type Array%20of%20BP%20Electric%20Generator%20Object%20References))
  (Variables|Default|SetGeneratorArray GeneratorArray)
  (for _index (range 0 (- (Utilities|Array|Length (Variables|Default|GetGeneratorArray)) 1))
    (Variables|Default|SetIndex _index)
    (Variables|Default|SetEG (Utilities|Array|Get(acopy) (Variables|Default|GetGeneratorArray) _index))
    (if (Variables|/Game/Blueprints/BP_ElectricGenerator.BP_ElectricGenerator_C|GetisActivated? (Utilities|Array|Get(acopy) (Variables|Default|GetGeneratorArray) _index))
      (if (== (Variables|/Game/Blueprints/BP_ElectricGenerator.BP_ElectricGenerator_C|GetOrderIndex (Variables|Default|GetEG)) 1)
        (Rendering|Material|SetMaterial (Variables|Default|Get1) 0 "/Game/Assets/ElectricalBox/ElectricalBoxLights_Mat_Inst_Inst.ElectricalBoxLights_Mat_Inst_Inst")
        (elif (== (Variables|/Game/Blueprints/BP_ElectricGenerator.BP_ElectricGenerator_C|GetOrderIndex (Variables|Default|GetEG)) 2)
          (Rendering|Material|SetMaterial (Variables|Default|Get2) 0 "/Game/Assets/ElectricalBox/ElectricalBoxLights_Mat_Inst_Inst.ElectricalBoxLights_Mat_Inst_Inst")
          (elif (== (Variables|/Game/Blueprints/BP_ElectricGenerator.BP_ElectricGenerator_C|GetOrderIndex (Variables|Default|GetEG)) 3)
            (Rendering|Material|SetMaterial (Variables|Default|Get3) 0 "/Game/Assets/ElectricalBox/ElectricalBoxLights_Mat_Inst_Inst.ElectricalBoxLights_Mat_Inst_Inst")
            (elif (== (Variables|/Game/Blueprints/BP_ElectricGenerator.BP_ElectricGenerator_C|GetOrderIndex (Variables|Default|GetEG)) 4)
              (Rendering|Material|SetMaterial (Variables|Default|Get4) 0 "/Game/Assets/ElectricalBox/ElectricalBoxLights_Mat_Inst_Inst.ElectricalBoxLights_Mat_Inst_Inst")
              (elif (== (Variables|/Game/Blueprints/BP_ElectricGenerator.BP_ElectricGenerator_C|GetOrderIndex (Variables|Default|GetEG)) 5)
                (Rendering|Material|SetMaterial (Variables|Default|Get5) 0 "/Game/Assets/ElectricalBox/ElectricalBoxLights_Mat_Inst_Inst.ElectricalBoxLights_Mat_Inst_Inst")
                (elif (== (Variables|/Game/Blueprints/BP_ElectricGenerator.BP_ElectricGenerator_C|GetOrderIndex (Variables|Default|GetEG)) 6)
                  (Rendering|Material|SetMaterial (Variables|Default|Get6) 0 "/Game/Assets/ElectricalBox/ElectricalBoxLights_Mat_Inst_Inst.ElectricalBoxLights_Mat_Inst_Inst"))))))))))

(fn ResetLight
  (Rendering|Material|SetMaterial (Variables|Default|Get1) 0 "/Game/Assets/ElectricalBox/ElectricalBoxLights_Mat_Inst_5.ElectricalBoxLights_Mat_Inst_5")
  (Rendering|Material|SetMaterial (Variables|Default|Get2) 0 "/Game/Assets/ElectricalBox/ElectricalBoxLights_Mat_Inst_4.ElectricalBoxLights_Mat_Inst_4")
  (Rendering|Material|SetMaterial (Variables|Default|Get3) 0 "/Game/Assets/ElectricalBox/ElectricalBoxLights_Mat_Inst.ElectricalBoxLights_Mat_Inst")
  (Rendering|Material|SetMaterial (Variables|Default|Get4) 0 "/Game/Assets/ElectricalBox/ElectricalBoxLights_Mat_Inst_3.ElectricalBoxLights_Mat_Inst_3")
  (Rendering|Material|SetMaterial (Variables|Default|Get5) 0 "/Game/Assets/ElectricalBox/ElectricalBoxLights_Mat_Inst_2.ElectricalBoxLights_Mat_Inst_2")
  (Rendering|Material|SetMaterial (Variables|Default|Get6) 0 "/Game/Assets/ElectricalBox/ElectricalBoxLights_Mat_Inst_6.ElectricalBoxLights_Mat_Inst_6")
  (for _array_element (Variables|Default|GetGeneratorArray)
    (Default|ResetEmissionValue _array_element)))