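; Trigger actor that checks whether wagons are connected when a BP_Train overlaps its box.
; The overlap event scans the Wagons array and clears a persistent Pass flag if any wagon reports not connected.
; If Pass survives the scan, it sets ChangeLane to false on EndTrack; otherwise it resets Pass to true for the next overlap.
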(event OnComponentBeginOverlap(Box)
  (params (OverlappedComponent :type Primitive%20Component%20Object%20Reference) (OtherActor :type Actor%20Object%20Reference) (OtherComp :type Primitive%20Component%20Object%20Reference) (OtherBodyIndex :type Integer) (bFromSweep :type Boolean) (SweepResult :type Hit%20Result%20Structure%20%28by%20ref%29))
  (Utilities|Casting|CastToBP_Train OtherActor)
  (for _array_element (Variables|Default|GetWagons)
    (if (Variables|Default|GetPass)
      (if (not (Variables|/Game/Blueprints/Train/BP_Train.BP_Train_C|GetIsConnected? _array_element))
        (Variables|Default|SetPass false))))
  (if (Variables|Default|GetPass)
    (Variables|/Game/Blueprints/Train/Track/BP_TrackSpline.BP_TrackSpline_C|SetChangeLane? (Variables|Default|GetEndTrack) false)
    (else
      (Variables|Default|SetPass true))))

(event EventBeginPlay)

(event Collision|EventActorBeginOverlap
  (params (OtherActor :type Actor%20Object%20Reference)))

(event EventTick
  (params (DeltaSeconds :type Float%20%28single-precision%29)))

(fn ConstructionScript)