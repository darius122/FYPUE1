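; BP_TrackSpline is a train track that builds its visible shape from a spline and can take over passing trains.
; The construction script adds a spline mesh per segment, matching endpoints and tangents to the spline points.
; When ChangeLane is set, overlapping its box switches a BP_Train onto this spline and recalculates the train's distance from the closest point to its world location.
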(event OnComponentBeginOverlap(Box)
  (params (OverlappedComponent :type Primitive%20Component%20Object%20Reference) (OtherActor :type Actor%20Object%20Reference) (OtherComp :type Primitive%20Component%20Object%20Reference) (OtherBodyIndex :type Integer) (bFromSweep :type Boolean) (SweepResult :type Hit%20Result%20Structure%20%28by%20ref%29))
  (if (Variables|Default|GetChangeLane?)
    (bind _asbp_train (Utilities|Casting|CastToBP_Train OtherActor))
    (bind _output_get (Variables|/Game/Blueprints/Train/BP_Train.BP_Train_C|SetTrack%20Spline _asbp_train (Variables|Default|GetTrackSpline)))
    ;[1 1 1] Get Position of Train Relative to the Spline Distance
    (Variables|/Game/Blueprints/Train/BP_Train.BP_Train_C|SetTrain%20Distance _asbp_train (Class|SplineComponent|GetDistanceAlongSplineatSplineInputKey _output_get (Class|SplineComponent|FindInputKeyClosesttoWorldLocation _output_get (Transformation|GetWorldLocation (Variables|/Game/Blueprints/Train/BP_Train.BP_Train_C|GetTrain _asbp_train)))))))

(event EventBeginPlay)

(event Collision|EventActorBeginOverlap
  (params (OtherActor :type Actor%20Object%20Reference)))

(event EventTick
  (params (DeltaSeconds :type Float%20%28single-precision%29)))

(fn ConstructionScript
  (bind _trackspline (Variables|Default|GetTrackSpline))
  (for _index (range 0 (- (Spline|GetNumberOfSplinePoints (Variables|Default|GetTrackSpline)) 2))
    (bind _returnvalue (AddComponent|AddSplineMeshComponent false))
    (Utilities|Array|Add (Variables|Default|GetSplineMeshArray) _returnvalue)
    (Transformation|AttachComponentToComponent _returnvalue 0 "None" "KeepRelative" "KeepRelative" "KeepRelative" true)
    (SplineMesh|SetStartandEnd _returnvalue (.Location (Spline|GetLocationandTangentatSplinePoint _trackspline _index "Local")) (.Tangent (Spline|GetLocationandTangentatSplinePoint _trackspline _index "Local")) (.Location (Spline|GetLocationandTangentatSplinePoint _trackspline (+ _index 1) "Local")) (.Tangent (Spline|GetLocationandTangentatSplinePoint _trackspline (+ _index 1) "Local")) true :!class /Script/Engine.SplineMeshComponent)))