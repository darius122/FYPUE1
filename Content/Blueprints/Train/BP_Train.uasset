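; BP_Train is a train that rides a track actor's spline, serving as either the lead train or a carriage-meshed wagon via IsWagon.
; While started, Tick advances distance by Speed, snaps the mesh to the spline when LaneState is moving, and loops or stops at track ends.
; Wagons use overlaps to start with another train's speed and loop setting, or halt and flag connected upon touching a stopped train.
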(event OnComponentBeginOverlap(Front)
  (params (OverlappedComponent :type Primitive%20Component%20Object%20Reference) (OtherActor :type Actor%20Object%20Reference) (OtherComp :type Primitive%20Component%20Object%20Reference) (OtherBodyIndex :type Integer) (bFromSweep :type Boolean) (SweepResult :type Hit%20Result%20Structure%20%28by%20ref%29))
  (if (Variables|Default|GetisWagon?)
    (if (Utilities|Enum|Equal(Enum) (Utilities|GetObjectName OtherComp) "Train")
      (bind _asbp_train (Utilities|Casting|CastToBP_Train OtherActor))
      (Variables|Default|SetisStart? true)
      (Variables|Default|SetSpeed (Class|MovementComponent|GetMaxSpeed (Pawn|GetMovementComponent _asbp_train)))
      (Variables|Default|SetisLoop? (Variables|BP_Train_C|GetisLoop? _asbp_train)))))

(event OnComponentBeginOverlap(ConnectTrain)
  (params (OverlappedComponent :type Primitive%20Component%20Object%20Reference) (OtherActor :type Actor%20Object%20Reference) (OtherComp :type Primitive%20Component%20Object%20Reference) (OtherBodyIndex :type Integer) (bFromSweep :type Boolean) (SweepResult :type Hit%20Result%20Structure%20%28by%20ref%29))
  (if (Variables|Default|GetisWagon?)
    (if (!= self OtherActor)
      (bind _asbp_train (Utilities|Casting|CastToBP_Train OtherActor))
      (if (not (Variables|BP_Train_C|GetisStart? _asbp_train))
        (Variables|Default|SetisStart? false)
        (Variables|Default|SetIsConnected? true)))))

(event EventBeginPlay
  (Variables|Default|SetTrack%20Spline (Variables|/Game/Blueprints/Train/Track/BP_TrackSpline.BP_TrackSpline_C|GetTrackSpline (Variables|Default|GetTrackActor)))
  ;[1 1 1] Get Position of Train Relative to the Spline Distance
  (Variables|Default|SetTrain%20Distance (Class|SplineComponent|GetDistanceAlongSplineatSplineInputKey (Variables|Default|GetTrack%20Spline) (Class|SplineComponent|FindInputKeyClosesttoWorldLocation (Variables|Default|GetTrack%20Spline) (Transformation|GetWorldLocation (Variables|Default|GetTrain))))))

(event Collision|EventActorBeginOverlap
  (params (OtherActor :type Actor%20Object%20Reference)))

(event EventTick
  (params (DeltaSeconds :type Float%20%28single-precision%29))
  (bind _train (Variables|Default|GetTrain))
  (if (Variables|Default|GetisStart?)
    (Variables|Default|SetTrain%20Distance (+ (Variables|Default|GetTrain%20Distance) (* DeltaSeconds (Variables|Default|GetSpeed))))
    (switch Utilities|FlowControl|Switch|SwitchonE_TrainMovementState (Variables|Default|GetLaneState)
      (:NewEnumerator0
        ;[1 1 1] Move Train
        (Transformation|SetWorldTransform _train (Math|Transform|MakeTransform (.location (Spline|GetTransformatDistanceAlongSpline (Variables|Default|GetTrack%20Spline) (Variables|Default|GetTrain%20Distance) "World" false)) (.rotation (Spline|GetTransformatDistanceAlongSpline (Variables|Default|GetTrack%20Spline) (Variables|Default|GetTrain%20Distance) "World" false)) (Transformation|GetWorldScale _train)) false false)
        ;[1 1 1] Set Max Speed of Pawn
        (Variables|/Script/Engine.FloatingPawnMovement|SetMaxSpeed (Variables|Default|GetFloatingPawnMovement) (Variables|Default|GetSpeed))
        ;[1 1 1] Loop Train
        (if (>= (Variables|Default|GetTrain%20Distance) (Spline|GetSplineLength (Variables|Default|GetTrack%20Spline)))
          (Variables|Default|SetCalc%20Distance 0.0)
          (if (Variables|Default|GetisLoop?) :!label _label
            (Variables|Default|SetTrain%20Distance (Variables|Default|GetCalc%20Distance))
            (else
              (Variables|Default|SetSpeed 0.0)
              (Variables|Default|SetisStart? false)))
          (elif (< (Variables|Default|GetTrain%20Distance) 0.0)
            (Variables|Default|SetCalc%20Distance (- (Spline|GetSplineLength (Variables|Default|GetTrack%20Spline)) (Variables|Default|GetTrain%20Distance)))
            (goto _label)))))))

(fn ConstructionScript
  (if (Variables|Default|GetisWagon?)
    (Components|StaticMesh|SetStaticMesh (Variables|Default|GetTrain) "/Game/Assets/Train/FYP_TrainCarriage_FBX.FYP_TrainCarriage_FBX")))