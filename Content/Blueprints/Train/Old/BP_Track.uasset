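; BP_Track is a rideable train track, building spline mesh segments along its spline in the construction script.
; When BP_FirstPersonCharacter overlaps RideCollision, it teleports above the lead mesh and the train starts.
; Tick advances a distance by Speed, placing the lead mesh and three carriages at fixed offsets along the spline.
; At spline's end the distance resets and the rider teleports to SpawnPoint, but IsInBox stays set, so the train keeps looping.
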(event OnComponentBeginOverlap(RideCollision)
  (params (OverlappedComponent :type Primitive%20Component%20Object%20Reference) (OtherActor :type Actor%20Object%20Reference) (OtherComp :type Primitive%20Component%20Object%20Reference) (OtherBodyIndex :type Integer) (bFromSweep :type Boolean) (SweepResult :type Hit%20Result%20Structure%20%28by%20ref%29))
  (Utilities|Casting|CastToBP_FirstPersonCharacter OtherActor)
  (Variables|Default|SetOther%20Actor OtherActor)
  (Variables|Default|SetisInBox true)
  (Development|PrintString "IN")
  (Transformation|SetActorTransform (Variables|Default|GetOther%20Actor) (Math|Transform|MakeTransform (+ (.location (Transformation|GetWorldTransform (Variables|Default|GetStaticMesh))) "0.000000,0.000000,500.000000") (.rotation (Transformation|GetWorldTransform (Variables|/Script/Engine.Actor|GetRootComponent (Variables|Default|GetOther%20Actor)))) "1.000000,1.000000,1.000000")))

(event EventBeginPlay)

(event Collision|EventActorBeginOverlap
  (params (OtherActor :type Actor%20Object%20Reference)))

(event EventTick
  (params (DeltaSeconds :type Float%20%28single-precision%29))
  (if (Variables|Default|GetisInBox)
    (Variables|Default|SetDistance (+ (* DeltaSeconds (Variables|Default|GetSpeed)) (Variables|Default|GetDistance)))
    (Variables|Default|SetFrontTrainDist (+ (Variables|Default|GetDistance) 2.9e+03))
    (Transformation|SetRelativeTransform (Variables|Default|GetStaticMesh) (Math|Transform|MakeTransform (.location (Spline|GetTransformatDistanceAlongSpline (Variables|Default|GetSpline) (+ (Variables|Default|GetDistance) 2.9e+03) "Local" false)) (.rotation (Spline|GetTransformatDistanceAlongSpline (Variables|Default|GetSpline) (+ (Variables|Default|GetDistance) 2.9e+03) "Local" false)) "1.000000,1.000000,1.000000") false false)
    (Transformation|SetRelativeTransform (Variables|Default|GetFYP_TrainCarriage_FBX) (Math|Transform|MakeTransform (.location (Spline|GetTransformatDistanceAlongSpline (Variables|Default|GetSpline) (+ (Variables|Default|GetDistance) 2e+03) "Local" false)) (.rotation (Spline|GetTransformatDistanceAlongSpline (Variables|Default|GetSpline) (+ (Variables|Default|GetDistance) 2e+03) "Local" false)) "1.000000,1.000000,1.000000") false false)
    (Transformation|SetRelativeTransform (Variables|Default|GetFYP_TrainCarriage_FBX1) (Math|Transform|MakeTransform (.location (Spline|GetTransformatDistanceAlongSpline (Variables|Default|GetSpline) (+ (Variables|Default|GetDistance) 1e+03) "Local" false)) (.rotation (Spline|GetTransformatDistanceAlongSpline (Variables|Default|GetSpline) (+ (Variables|Default|GetDistance) 1e+03) "Local" false)) "1.000000,1.000000,1.000000") false false)
    (Transformation|SetRelativeTransform (Variables|Default|GetFYP_TrainCarriage_FBX2) (Math|Transform|MakeTransform (.location (Spline|GetTransformatDistanceAlongSpline (Variables|Default|GetSpline) (Variables|Default|GetDistance) "Local" false)) (.rotation (Spline|GetTransformatDistanceAlongSpline (Variables|Default|GetSpline) (Variables|Default|GetDistance) "Local" false)) "1.000000,1.000000,1.000000") false false)
    (if (!= (Variables|Default|GetOther%20Actor) 0)
      (if (>= (Variables|Default|GetFrontTrainDist) (Spline|GetSplineLength (Variables|Default|GetSpline)))
        (Variables|Default|SetDistance 0.0)
        (Transformation|SetActorTransform (Variables|Default|GetOther%20Actor) (Math|Transform|MakeTransform (+ (Transformation|GetWorldLocation (Variables|Default|GetSpawnPoint)) "0.000000,0.000000,70.000000") "0, 0, 0" "1.000000,1.000000,1.000000"))))))

(fn ConstructionScript
  (bind _meshsize (Variables|Default|GetMeshSize))
  (bind _spline (Variables|Default|GetSpline))
  (bind _spline_2 (Variables|Default|GetSpline))
  (for _index (range 0 (Math|Float|Truncate (/ (Spline|GetSplineLength (Variables|Default|GetSpline)) (Variables|Default|GetMeshSize))))
    (if (not (> (+ (* _index _meshsize) _meshsize) (Spline|GetSplineLength (Variables|Default|GetSpline))))
      (bind _returnvalue (AddComponent|AddSplineMeshComponent false))
      (SplineMesh|SetStartandEnd _returnvalue (Spline|GetLocationatDistanceAlongSpline _spline_2 (* _index _meshsize) "Local") (Math|Vector|ClampVectorSize (Spline|GetTangentatDistanceAlongSpline _spline_2 (* _index _meshsize) "Local") 0.0 (Variables|Default|GetMeshSize)) (Spline|GetLocationatDistanceAlongSpline _spline (+ (* _index _meshsize) _meshsize) "Local") (Math|Vector|ClampVectorSize (Spline|GetTangentatDistanceAlongSpline _spline (+ (* _index _meshsize) _meshsize) "Local") 0.0 (Variables|Default|GetMeshSize)) true :!class /Script/Engine.SplineMeshComponent))))