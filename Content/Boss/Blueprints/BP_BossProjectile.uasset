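; BP_BossProjectile is a boss projectile that homes in on the player and damages them on contact.
; After a short delay from BeginPlay, GoToPlayer sets the first BP_FirstPersonCharacter found as the ProjectileMovement homing target.
; Box overlap with that character class applies fixed damage and destroys the projectile.
; A PlayMontage call sits unconnected and never runs.
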(event OnComponentBeginOverlap(Box)
  (params (OverlappedComponent :type Primitive%20Component%20Object%20Reference) (OtherActor :type Actor%20Object%20Reference) (OtherComp :type Primitive%20Component%20Object%20Reference) (OtherBodyIndex :type Integer) (bFromSweep :type Boolean) (SweepResult :type Hit%20Result%20Structure%20%28by%20ref%29))
  (bind _asbp_first_person_character (Utilities|Casting|CastToBP_FirstPersonCharacter OtherActor))
  (Game|Damage|ApplyDamage _asbp_first_person_character 1e+01 0 0)
  (Actor|DestroyActor))

(event EventBeginPlay
  ;[1 1 1] play animation then fly to player
  (Utilities|FlowControl|Delay 2.0)
  (CallFunction|GotoPlayer))

(fn ConstructionScript)

(fn GotoPlayer
  (bind _outactors (Actor|GetAllActorsOfClass "/Game/FirstPerson/Blueprints/BP_FirstPersonCharacter.BP_FirstPersonCharacter_C"))
  (Variables|/Script/Engine.ProjectileMovementComponent|SetHomingTargetComponent (Variables|Default|GetProjectileMovement) (Variables|/Script/Engine.Actor|GetRootComponent (Utilities|Array|Get(acopy) _outactors))))