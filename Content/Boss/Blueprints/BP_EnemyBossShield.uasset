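; Boss shield actor that picks one of three elements at random on BeginPlay and absorbs head projectiles of that element.
; A sphere overlap with a matching BP_EnemyHeadProjectile destroys the projectile and decrements shield health, while other elements are left untouched.
; When health reaches zero or below, it calls StopHealing on the referenced boss.
; Tick prints shield health on screen every frame.
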(event OnComponentBeginOverlap(Sphere)
  (params (OverlappedComponent :type Primitive%20Component%20Object%20Reference) (OtherActor :type Actor%20Object%20Reference) (OtherComp :type Primitive%20Component%20Object%20Reference) (OtherBodyIndex :type Integer) (bFromSweep :type Boolean) (SweepResult :type Hit%20Result%20Structure%20%28by%20ref%29))
  (bind _asbp_enemy_head_projectile (Utilities|Casting|CastToBP_EnemyHeadProjectile OtherActor))
  (if (Utilities|Enum|Equal(Enum) (Variables|Default|GetShield%20Element) (Variables|/Game/FirstPerson/Blueprints/Weapon/Launcher/Projectile/BP_EnemyHeadProjectile.BP_EnemyHeadProjectile_C|GetHeadProjectileElement _asbp_enemy_head_projectile))
    (Actor|DestroyActor _asbp_enemy_head_projectile)
    (bind _result (Math|Integer|DecrementInt (Variables|Default|GetShield%20Health))
      (:%20%20
        (bind _output_get (Variables|Default|SetShield%20Health _result))
        (if (<= _output_get 0)
          (Default|StopHealing (Variables|Default|GetBoss%20REF)))))))

(event EventBeginPlay
  (switch int (Math|Random|RandomIntegerinRange 0 2)
    (:0
      (Variables|Default|SetShield%20Element "NewEnumerator0"))
    (:1
      (Variables|Default|SetShield%20Element "NewEnumerator1"))
    (:2
      (Variables|Default|SetShield%20Element "NewEnumerator2"))))

(event Collision|EventActorBeginOverlap
  (params (OtherActor :type Actor%20Object%20Reference)))

(event EventTick
  (params (DeltaSeconds :type Float%20%28single-precision%29))
  (Development|PrintString (Utilities|String|ToString(Integer) (Variables|Default|GetShield%20Health))))

(fn ConstructionScript)