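; Projectile for the boss rain attack that explodes when its box overlaps a BP_ProjectileSpawnArea actor.
; On overlap it runs a sphere overlap for pawns at that area's sphere and damages the first result if it is the first-person character.
; It then spawns an explosion emitter there and destroys both the spawn area and itself.
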(event OnComponentBeginOverlap(Box)
  (params (OverlappedComponent :type Primitive%20Component%20Object%20Reference) (OtherActor :type Actor%20Object%20Reference) (OtherComp :type Primitive%20Component%20Object%20Reference) (OtherBodyIndex :type Integer) (bFromSweep :type Boolean) (SweepResult :type Hit%20Result%20Structure%20%28by%20ref%29))
  (bind _asbp_projectile_spawn_area (Utilities|Casting|CastToBP_ProjectileSpawnArea OtherActor))
  (bind (_outactors _returnvalue) (Collision|SphereOverlapActors (Transformation|GetWorldLocation (Variables|/Game/Boss/Blueprints/BP_ProjectileSpawnArea.BP_ProjectileSpawnArea_C|GetSphere _asbp_projectile_spawn_area)) 2.5e+02 (Utilities|Array|MakeArray "ObjectTypeQuery3") 0))
  (if _returnvalue
    (bind _asbp_first_person_character (Utilities|Casting|CastToBP_FirstPersonCharacter (Utilities|Array|Get(acopy) _outactors))
      (:then
        (Game|Damage|ApplyDamage _asbp_first_person_character 2e+01 0 0))
      (:CastFailed
        _)))
  (Effects|SpawnEmitteratLocation "/Game/StarterContent/Particles/P_Explosion.P_Explosion" (Transformation|GetWorldLocation (Variables|/Game/Boss/Blueprints/BP_ProjectileSpawnArea.BP_ProjectileSpawnArea_C|GetSphere _asbp_projectile_spawn_area)) "0, 0, 0" "3.000000,3.000000,3.000000")
  (Actor|DestroyActor OtherActor)
  (Actor|DestroyActor))

(event EventBeginPlay)

(event Collision|EventActorBeginOverlap
  (params (OtherActor :type Actor%20Object%20Reference)))

(event EventTick
  (params (DeltaSeconds :type Float%20%28single-precision%29)))

(fn ConstructionScript)